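; Player controller for the 2D framework game that routes move, jump and timed attack input to the cached BP_CH_PawnBase.
; Consume/Use Item runs both gamepad and keyboard handlers, mapping the key's display name to one of three HUD hotbar slots.
; The slot's ItemID looks up DT_ItemData; a consumable Potion adds health and is removed from the pawn's inventory.
; Pause freezes the game and opens WBP_PauseMenu with UI-only input.
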(event `self.ReceiveBeginPlay`
  (bind _returnvalue (`GameplayStatics.GetPlayerPawn` 0))
  (`/Engine/EditorBlueprintResources/StandardMacros.IsValid` _returnvalue
    (:`Is Valid`
      (bind _asbp_ch_pawn_base (cast `/Game/2DFramework/Blueprints/Core/BP_CH_PawnBase` _returnvalue))
      (set `self.As BP CH Pawn` _asbp_ch_pawn_base)
      (`WidgetBlueprintLibrary.SetInputMode_GameOnly` self))))

(event `InputAction|Consume/Use Item`
  (params (Key :type "Key Structure"))
  (:`Pressed`
    (`self.Gamepad Key's Function` Key)
    (`self.Keyboard & Mouse Key's Function` Key)))

(event `InputAction|Attack`
  (params (Key :type "Key Structure"))
  ;[0 0 0 0] Attack Function
  (:`Pressed`
    (if (not (`NavMovementComponent.IsFalling` (`Character.CharacterMovement` (`self.As BP CH Pawn`))))
      (`/Game/2DFramework/Blueprints/Core/BP_CH_PawnBase.Attack Function` (`self.As BP CH Pawn`))
      (`KismetSystemLibrary.Delay` 0.5)
      (`/Game/2DFramework/Blueprints/Core/BP_CH_PawnBase.Stop Attack Function` (`self.As BP CH Pawn`)))))

(event `InputAxis|Move Forward / Backward`
  (params (AxisValue :type "Float (single-precision)"))
  (bind _as_bp_ch_pawn (`self.As BP CH Pawn`))
  ;[0 0 0 0] Move Function
  (`/Engine/EditorBlueprintResources/StandardMacros.IsValid` _as_bp_ch_pawn
    (:`Is Valid`
      (`/Game/2DFramework/Blueprints/Core/BP_CH_PawnBase.Move Function` _as_bp_ch_pawn AxisValue))))

(event `InputAction|Jump`
  (params (Key :type "Key Structure"))
  ;[0 0 0 0] Jump Function
  (:`Pressed`
    (`Character.Jump` (`self.As BP CH Pawn`))))

(event `InputAction|Pause` :paused true
  (params (Key :type "Key Structure"))
  ;[0 0 0 0] Pause Input | Pause Game
  (:`Pressed`
    (`GameplayStatics.SetGamePaused` true)
    (set `self.bShowMouseCursor` true)
    (`WidgetBlueprintLibrary.SetInputMode_UIOnlyEx` self null)
    (bind _returnvalue (`|CreateWidget` "/Game/2DFramework/Blueprints/UI/PauseMenu/WBP_PauseMenu.WBP_PauseMenu_C" null self))
    (`UserWidget.AddToViewport` _returnvalue 0)))

(fn `Access The Inventory & Remove The Item`
  (for (_array_element _array_index) (`/Game/2DFramework/Systems/InventorySystem/Blueprints/Components/BPC_InventorySTM.Inventory Content` (`/Game/2DFramework/Blueprints/Core/BP_CH_PawnBase.BPC_InventorySTM` (`self.As BP CH Pawn`)))
    (if (== (`.ItemID_4_6C53946244414507F6CC6A88B2CD4871` (break `/Game/2DFramework/Systems/InventorySystem/Data/S_SlotStruct` _array_element)) (`self.Item ID`))
      (`/Game/2DFramework/Systems/InventorySystem/Blueprints/Components/BPC_InventorySTM.Remove From Inventory` (`/Game/2DFramework/Blueprints/Core/BP_CH_PawnBase.BPC_InventorySTM` (`self.As BP CH Pawn`)) _array_index false true))))

(fn `Gamepad Key's Function`
  (params (Key :type "Key Structure (by ref)"))
  (bind _wbp_game (`/Game/2DFramework/Blueprints/Core/BP_HUD_Game.WBP Game` (`self.GetHUDRef`)))
  (`self.Get Input Key From Gamepad` Key)
  (bind _aswbp_hotbar_slot (cast `/Game/2DFramework/Systems/InventorySystem/UI/Hotbar/WBP_HotbarSlot` (`|GetArrayItem` (`|MakeArray` (`/Game/2DFramework/Blueprints/UI/Player/WBP_Game.WBP_HotbarSlot` _wbp_game) (`/Game/2DFramework/Blueprints/UI/Player/WBP_Game.WBP_HotbarSlot_1` _wbp_game) (`/Game/2DFramework/Blueprints/UI/Player/WBP_Game.WBP_HotbarSlot_2` _wbp_game) :!type "Widget Object Reference") (- (`self.Input Key`) 1))))
  (bind _output_get (set `self.Item ID` (`/Game/2DFramework/Systems/InventorySystem/UI/Hotbar/WBP_HotbarSlot.Item ID` _aswbp_hotbar_slot)))
  (bind _returnvalue (`|GetDataTableRow` "/Game/2DFramework/Systems/InventorySystem/Data/DT_ItemData.DT_ItemData" _output_get)
    (:`then`
      (bind ((`Consumable?_22_7B1A0D22493C4F2A10F77190D51AF4BD` _consumable_) (`Consumable_21_16A823234D05BA200A0B479AEEFC4451` _consumable)) (break `/Game/2DFramework/Systems/InventorySystem/Data/S_ItemStruct` _returnvalue))
      (if _consumable_
        (switch `name` (`self.Item ID`)
          (:`Potion`
            (`/Game/2DFramework/Blueprints/Components/AC_StatSystem.Add Health` (`/Game/2DFramework/Blueprints/Core/BP_CH_PawnBase.AC_HPSystem` (`self.As BP CH Pawn`)) false _consumable)
            (`self.Access The Inventory & Remove The Item`)))))))

(fn `Get Input Key From Gamepad`
  (params (Key :type "Key Structure (by ref)"))
  (switch `string` (`KismetTextLibrary.Conv_TextToString` (`KismetInputLibrary.Key_GetDisplayName` Key))
    (:`Gamepad Face Button Top`
      (set `self.Input Key` 1))
    (:`Gamepad Face Button Right`
      (set `self.Input Key` 2))
    (:`Gamepad Face Button Bottom`
      (set `self.Input Key` 3))
    (:`Gamepad Face Button Left`
      (set `self.Input Key` 4))
    (:`Gamepad D-pad Up`
      (set `self.Input Key` 5))
    (:`Gamepad D-pad Right`
      (set `self.Input Key` 6))
    (:`Gamepad D-pad Down`
      (set `self.Input Key` 7))
    (:`Gamepad D-pad Left`
      (set `self.Input Key` 8))))

(fn `GetHUDRef`
  (returns (`As BP HUD Game` :type "/Game/2DFramework/Blueprints/Core/BP_HUD_Game Object Reference"))
  (`self.As BP HUD Game`
    (:`then`
      _)
    (:`else`
      (bind _asbp_hud_game (cast `/Game/2DFramework/Blueprints/Core/BP_HUD_Game` (`self.GetHUD`)))
      (set `self.As BP HUD Game` _asbp_hud_game)))
  (return (`self.As BP HUD Game`)))

(fn `Keyboard & Mouse Key's Function`
  (params (Key :type "Key Structure (by ref)"))
  (bind _wbp_game (`/Game/2DFramework/Blueprints/Core/BP_HUD_Game.WBP Game` (`self.GetHUDRef`)))
  (bind _aswbp_hotbar_slot (cast `/Game/2DFramework/Systems/InventorySystem/UI/Hotbar/WBP_HotbarSlot` (`|GetArrayItem` (`|MakeArray` (`/Game/2DFramework/Blueprints/UI/Player/WBP_Game.WBP_HotbarSlot` _wbp_game) (`/Game/2DFramework/Blueprints/UI/Player/WBP_Game.WBP_HotbarSlot_1` _wbp_game) (`/Game/2DFramework/Blueprints/UI/Player/WBP_Game.WBP_HotbarSlot_2` _wbp_game)) (- (`KismetStringLibrary.Conv_StringToInt` (`KismetTextLibrary.Conv_TextToString` (`KismetInputLibrary.Key_GetDisplayName` Key))) 1))))
  (bind _output_get (set `self.Item ID` (`/Game/2DFramework/Systems/InventorySystem/UI/Hotbar/WBP_HotbarSlot.Item ID` _aswbp_hotbar_slot)))
  (bind _returnvalue (`|GetDataTableRow` "/Game/2DFramework/Systems/InventorySystem/Data/DT_ItemData.DT_ItemData" _output_get)
    (:`then`
      (bind ((`Consumable?_22_7B1A0D22493C4F2A10F77190D51AF4BD` _consumable_) (`Consumable_21_16A823234D05BA200A0B479AEEFC4451` _consumable)) (break `/Game/2DFramework/Systems/InventorySystem/Data/S_ItemStruct` _returnvalue))
      (if _consumable_
        (switch `name` (`self.Item ID`)
          (:`Potion`
            (`/Game/2DFramework/Blueprints/Components/AC_StatSystem.Add Health` (`/Game/2DFramework/Blueprints/Core/BP_CH_PawnBase.AC_HPSystem` (`self.As BP CH Pawn`)) false _consumable)
            ;[0.2855 0.4571 1] Access the contents of the inventory to remove the item we have consumed,
            ; in this case the potion. But it is a reusable function for all types of items we create.
            ;
            ; Acceder al contenido del inventario para remover de él, el item que hayamos consumido,
            ; en este caso la poción. Pero es una función reutilizable en todo tipos de items que creemos.
            (`self.Access The Inventory & Remove The Item`)))))))

(fn `UserConstructionScript`)