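; Base player character for the 2D framework, with side-view movement, capsule-trace melee attacks, interaction, dialogue and inventory, creating the player save game on BeginPlay.
; ACHPSystem takes incoming damage and holds mana, which looping timers drain while sprinting and refill afterwards.
; Overlaps and interface messages drive dialogue and interactables, while input opens inventory or chest widgets.
; Any key press switches on-screen input icons between gamepad and keyboard.
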(event `self.ReceiveBeginPlay`
  (`/Game/2DFramework/Blueprints/BP_GI_Main.Create Player SaveGame` (`self.GetGIRef`))
  (`self.Restore Mana`))

(event `self.ReceiveAnyDamage`
  (params (Damage :type "Float (single-precision)") (DamageType :type "DamageType Object Reference") (InstigatedBy :type "Controller Object Reference") (DamageCauser :type "Actor Object Reference"))
  (`/Game/2DFramework/Blueprints/Components/AC_StatSystem.Get Hurt` (`self.AC_HPSystem`) false Damage))

(event `InputAction|OpenInventory`
  (params (Key :type "Key Structure"))
  (:`Pressed`
    (bind _returnvalue (`|CreateWidget` "/Game/2DFramework/Systems/InventorySystem/UI/Grids/WBP_InventoryPlayer.WBP_InventoryPlayer_C"))
    (`UserWidget.AddToPlayerScreen` _returnvalue 0)
    (`MovementComponent.StopMovementImmediately` (`self.CharacterMovement`))))

(event `InputAction|OpenChest`
  (params (Key :type "Key Structure"))
  (:`Pressed`
    (bind _chesttoopen (`self.ChestToOpen`)
      (:`then`
        (bind _returnvalue (`|CreateWidget` "/Game/2DFramework/Systems/InventorySystem/UI/Grids/WBP_InventoryContainer.WBP_InventoryContainer_C" null (`/Game/2DFramework/Systems/InventorySystem/Blueprints/Containers/BP_InteractableChest.BPC_InventorySTM` _chesttoopen) _chesttoopen))
        (`UserWidget.AddToPlayerScreen` _returnvalue 0)
        (`MovementComponent.StopMovementImmediately` (`self.CharacterMovement`))
        (`PaperSpriteComponent.SetSprite` (`/Game/2DFramework/Systems/InventorySystem/Blueprints/Containers/BP_InteractableChest.PaperSprite` _chesttoopen) "/Game/2DFramework/Resources/Sprites/Chest/S_Chest_Open.S_Chest_Open"))
      (:`else`))))

(event `InputAction|Interact`
  (params (Key :type "Key Structure"))
  (:`Pressed`
    (`|ExecutionSequence`
      (:`then_0`
        (bind _active_interactable (`self.Active Interactable`)
          (:`then`
            (message `/Game/2DFramework/Systems/InteractionSystem/BPI_InteractionSystem.Interact` _active_interactable))
          (:`else`)))
      (:`then_1`
        (`/Game/2DFramework/Systems/InventorySystem/Blueprints/Components/BPC_InventorySTM.Interact Input` (`self.BPC_InventorySTM`))))))

(event `Key|AnyKey` :overrideparent false
  (params (Key :type "Key Structure"))
  ;[0 0.3813 0.8714] Change UI Icons
  (:`Pressed`
    (bind _foundwidgets (`WidgetBlueprintLibrary.GetAllWidgetsOfClass` "/Game/2DFramework/Blueprints/UI/WBP_InputImage.WBP_InputImage_C" false))
    (for _array_element _foundwidgets
      (if (`KismetInputLibrary.Key_IsGamepadKey` Key)
        (`/Game/2DFramework/Blueprints/UI/WBP_InputImage.Refresh Inputs Icons` _array_element true)
        (else
          (`/Game/2DFramework/Blueprints/UI/WBP_InputImage.Refresh Inputs Icons` _array_element false))))))

(event `self.DialogueInteract.OnComponentBeginOverlap`
  (params (OverlappedComponent :type "PrimitiveComponent Object Reference") (OtherActor :type "Actor Object Reference") (OtherComp :type "PrimitiveComponent Object Reference") (OtherBodyIndex :type Integer) (bFromSweep :type Boolean) (SweepResult :type "HitResult Structure (by ref)"))
  (if (!= OtherActor self)
    (if (`KismetSystemLibrary.DoesImplementInterface` OtherActor "/Game/2DFramework/Systems/AdvancedDialogueSystem/Blueprints/BPI_Interact.BPI_Interact_C")
      (`/Engine/EditorBlueprintResources/StandardMacros.IsValid` (`self.Interactable`)
        (:`Is Valid`
          (message `/Game/2DFramework/Systems/AdvancedDialogueSystem/Blueprints/BPI_Interact.SetInteractableState` (`self.Interactable`) false)
          (set `self.Interactable` null))
        (:`Is Not Valid`
          _))
      (set `self.Interactable` OtherActor)
      (message `/Game/2DFramework/Systems/AdvancedDialogueSystem/Blueprints/BPI_Interact.SetInteractableState` (`self.Interactable`) true))))

(event `self.DialogueInteract.OnComponentEndOverlap`
  (params (OverlappedComponent :type "PrimitiveComponent Object Reference") (OtherActor :type "Actor Object Reference") (OtherComp :type "PrimitiveComponent Object Reference") (OtherBodyIndex :type Integer))
  (if (and (!= OtherActor self) (== (`self.Interactable`) OtherActor))
    (message `/Game/2DFramework/Systems/AdvancedDialogueSystem/Blueprints/BPI_Interact.SetInteractableState` (`self.Interactable`) false)
    (set `self.Interactable` null)))

(event `Key|E`
  (params (Key :type "Key Structure"))
  (bind _returnvalue (`GameplayStatics.GetPlayerController` 0))
  (:`Pressed`
    (`/Engine/EditorBlueprintResources/StandardMacros.IsValid` (`self.Interactable`)
      (:`Is Valid`
        (message `/Game/2DFramework/Systems/AdvancedDialogueSystem/Blueprints/BPI_Interact.Interact` (`self.Interactable`) self)
        (`WidgetBlueprintLibrary.SetInputMode_UIOnlyEx` _returnvalue null)
        (set `PlayerController.bShowMouseCursor` true _returnvalue)))))

(event `InputAction|Sprint`
  (params (Key :type "Key Structure"))
  (:`Pressed`
    (if (>= (`/Game/2DFramework/Blueprints/Components/AC_StatSystem.Mana` (`self.AC_HPSystem`)) 10.0)
      (set `CharacterMovementComponent.MaxWalkSpeed` 1000.0 (`self.CharacterMovement`))
      (set `self.Player Is Sprinting?` true)
      (bind _returnvalue (`KismetSystemLibrary.K2_SetTimerDelegate` (delegate `Subtract Mana`) 0.3 true))
      (else
        (`self.Restore Mana`))))
  (:`Released`
    (set `self.Player Is Sprinting?` false)
    ;[1 1 1] Finish Sprint
    (set `CharacterMovementComponent.MaxWalkSpeed` 600.0 (`self.CharacterMovement`))
    (`KismetSystemLibrary.K2_ClearAndInvalidateTimerHandle` _returnvalue)
    (`KismetSystemLibrary.Delay` 5.0)
    (`self.Restore Mana`)))

(event `Subtract Mana`
  (bind _ac_hpsystem (`self.AC_HPSystem`))
  (`/Game/2DFramework/Blueprints/Components/AC_StatSystem.Subtract Mana` _ac_hpsystem 3.0)
  (if (<= (`/Game/2DFramework/Blueprints/Components/AC_StatSystem.Mana` _ac_hpsystem) 0.0)
    ;[1 1 1] Finish Sprint
    (set `CharacterMovementComponent.MaxWalkSpeed` 600.0 (`self.CharacterMovement`))
    (`KismetSystemLibrary.K2_ClearAndInvalidateTimerHandle` (stale `InputAction|Sprint` _returnvalue))
    (`KismetSystemLibrary.Delay` 5.0)
    (`self.Restore Mana`)))

(event `Restore Mana`
  (bind _returnvalue (`KismetSystemLibrary.K2_SetTimerDelegate` (delegate `Mana Restore Timer`) 0.3 true)))

(event `Mana Restore Timer`
  (bind _ac_hpsystem (`self.AC_HPSystem`))
  (if (`self.Player Is Sprinting?`)
    (`KismetSystemLibrary.K2_ClearAndInvalidateTimerHandle` (stale `Restore Mana` _returnvalue))
    (else
      (`/Game/2DFramework/Blueprints/Components/AC_StatSystem.Add Mana` _ac_hpsystem 7.0)
      (if (>= (`/Game/2DFramework/Blueprints/Components/AC_StatSystem.Mana` _ac_hpsystem) 100.0)
        (`KismetSystemLibrary.K2_ClearAndInvalidateTimerHandle` (stale `Restore Mana` _returnvalue))))))

(fn `Add Interactable`
  (params (`Active Interactable` :type "Actor Object Reference"))
  (set `self.Active Interactable` `Active Interactable`))

(fn `Attack Function`
  (bind _returnvalue (`self.K2_GetActorLocation`))
  (bind (_returnvalue_roll _returnvalue_pitch _returnvalue_yaw) (`KismetMathLibrary.BreakRotator` (`SceneComponent.K2_GetComponentRotation` (`self.Sprite`))))
  (`MovementComponent.StopMovementImmediately` (`self.CharacterMovement`))
  (bind (_outhit _returnvalue_2) (`KismetSystemLibrary.CapsuleTraceSingle` _returnvalue (+ _returnvalue (`KismetMathLibrary.MakeVector` (select `bool` (!= _returnvalue_yaw 180.0) :`false` -100.0 :`true` 100.0 :!type "Float (single-precision)"))) 25.0 25.0 "TraceTypeQuery1"))
  (bind _output_get (set `self.Hit Actor Struct` (make `/Game/2DFramework/Data/Structs/Player/S_HitActorStruct` _outhit _returnvalue_2)))
  (set `/Game/2DFramework/Blueprints/Components/BPC_AnimComponent.Is Attack?` true (`self.BPC_AnimComponent`))
  (`GameplayStatics.ApplyDamage` (`.HitActor` (`GameplayStatics.BreakHitResult` (`.HitResult_3_89D5B7374B3E523E63730F880BAC1030` (break `/Game/2DFramework/Data/Structs/Player/S_HitActorStruct` _output_get)))) (`self.Player Damage`)))

(fn `GetGIRef`
  (returns (`As BP GI Main` :type "/Game/2DFramework/Blueprints/BP_GI_Main Object Reference"))
  (`self.As BP GI Main`
    (:`then`
      _)
    (:`else`
      (bind _asbp_gi_main (cast `/Game/2DFramework/Blueprints/BP_GI_Main` (`GameplayStatics.GetGameInstance`)))
      (set `self.As BP GI Main` _asbp_gi_main)))
  (return (`self.As BP GI Main`)))

(fn `Move Function`
  (params (`Action Value` :type "Float (double-precision)"))
  (`PawnMovementComponent.AddInputVector` (`Character.CharacterMovement` (`GameplayStatics.GetPlayerCharacter` 0)) (`KismetMathLibrary.MakeVector` `Action Value`) false) ; Node to add motion in the X-Axis\n\nNodo para añadir movimiento en el eje X
  (if (!= `Action Value` 0.0)
    (`SceneComponent.K2_SetRelativeRotation` (`self.Sprite`) (`KismetMathLibrary.MakeRotator` 0.0 0.0 (select `bool` (> (`local.Action Value`) 0.0) :`true` -180.0 :!type "Float (single-precision)")) false false) ; Rotate the player according to the "Action Value"\n\nRotar el jugador en función del "Action Value"
  ))

(fn `Remove Interactable`
  (params (Interactable :type "Actor Object Reference"))
  (if (== Interactable (`self.Active Interactable`))
    (set `self.Active Interactable` null)))

(fn `Stop Attack Function`
  (set `/Game/2DFramework/Blueprints/Components/BPC_AnimComponent.Is Attack?` false (`self.BPC_AnimComponent`)))

(fn `UserConstructionScript`)