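; Game Instance for the 2D framework that manages saving and loading of player and enemy state.
; On Init it loads or creates the BP_SG_Player save object and caches it for the other functions.
; Save functions write player health and location, plus an actor-keyed map of enemy states, to the slot; load functions reapply them to pawns and stat components.
; NewGame deletes the "PlayerData" slot and opens the given level.
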(event `Create Player SaveGame`
  (bind _player_slot_name (`self.Player Slot Name`))
  ;[0.2558 1 0.2083 0] INIT Event | Runs at startup to create the save objects.
  (bind _returnvalue (`GameplayStatics.DoesSaveGameExist` (`self.Player Slot Name`) :!label _label)) ; Is there a Save Game with the name "Data" Slot?
  (if _returnvalue
    ;;[0 0 0 0 13] Is there a Save Game with the slot name "Data"? I load it, cast it to my save game and save it in variable
    (bind _returnvalue_2 (`GameplayStatics.LoadGameFromSlot` (`self.Player Slot Name`)))
    (bind _asbp_sg_player (cast `/Game/2DFramework/Blueprints/SaveGame/BP_SG_Player` _returnvalue_2))
    (bind _output_get (set `self.As BP SG Player` _asbp_sg_player))
    (`GameplayStatics.SaveGameToSlot` _output_get _player_slot_name)
    (else
      ;;[0 0 0 0 13] Does it not exist? I create it and keep it in variable
      (bind _returnvalue_3 (`GameplayStatics.CreateSaveGameObject` "/Game/2DFramework/Blueprints/SaveGame/BP_SG_Player.BP_SG_Player_C"))
      (bind _output_get_2 (set `self.As BP SG Player` _returnvalue_3))
      (`GameplayStatics.SaveGameToSlot` _output_get_2 _player_slot_name))))

(event `self.ReceiveInit`
  ;[0.2558 1 0.2083 0] INIT Event | Runs at startup to create the save objects.
  (bind _returnvalue (`GameplayStatics.GetCurrentLevelName` true))
  (switch `string` _returnvalue
    (:`L_Forest`
      (goto _label))))

(fn `Load Enemies`
  (bind _enemy_config (`/Game/2DFramework/Blueprints/SaveGame/BP_SG_Player.Enemy Config` (`self.As BP SG Player`)))
  (bind _keys (`BlueprintMapLibrary.Map_Keys` _enemy_config))
  (for _array_element _keys
    (bind _asbp_enemy_base (cast `/Game/2DFramework/Systems/ArtificialIntelligenceSystem/BP_EnemyBase` _array_element))
    (bind _value (`BlueprintMapLibrary.Map_Find` _enemy_config _array_element))
    (`Actor.K2_SetActorLocation` _asbp_enemy_base (`.Location_5_D6BB749F47B039A663299D81CE5DDDAD` (break `/Game/2DFramework/Data/Structs/Enemy/S_SaveGameEnemy` _value)) false false)
    (set `/Game/2DFramework/Blueprints/Components/AC_StatSystem.Health` (break `/Game/2DFramework/Data/Structs/Enemy/S_SaveGameEnemy` _value) (`/Game/2DFramework/Systems/ArtificialIntelligenceSystem/BP_EnemyBase.AC_StatSystem` _asbp_enemy_base))))

(fn `Load Game`
  (bind _returnvalue (`GameplayStatics.GetPlayerPawn` 0))
  (bind _location (`/Game/2DFramework/Blueprints/SaveGame/BP_SG_Player.Location` (`self.As BP SG Player`)))
  (if (!= _location (0.0 0.0 0.0))
    (`Actor.K2_SetActorLocation` _returnvalue _location false false)
    (bind _asbp_ch_pawn_base (cast `/Game/2DFramework/Blueprints/Core/BP_CH_PawnBase` _returnvalue))
    (set `/Game/2DFramework/Blueprints/Components/AC_StatSystem.Health` (`/Game/2DFramework/Blueprints/SaveGame/BP_SG_Player.Health` (`self.As BP SG Player`)) (`/Game/2DFramework/Blueprints/Core/BP_CH_PawnBase.AC_HPSystem` _asbp_ch_pawn_base))))

(fn `New Game`
  (params (`Level to Open` :type "World Soft Object Reference") (`Level Options` :type String))
  (`Actor.K2_SetActorLocation` (`GameplayStatics.GetPlayerPawn` 0) (0.0 0.0 0.0) false false)
  (`GameplayStatics.DeleteGameInSlot` "PlayerData")
  (`GameplayStatics.OpenLevelBySoftObjectPtr` `Level to Open` true `Level Options`))

(fn `Save Enemies `
  (params (Actor :type "Actor Object Reference") (Health :type "Float (double-precision)") (Location :type "Vector Structure"))
  (bind _as_bp_sg_player (`self.As BP SG Player`))
  (`BlueprintMapLibrary.Map_Add` (`/Game/2DFramework/Blueprints/SaveGame/BP_SG_Player.Enemy Config` _as_bp_sg_player) Actor (make `/Game/2DFramework/Data/Structs/Enemy/S_SaveGameEnemy` Health Location))
  (`GameplayStatics.SaveGameToSlot` _as_bp_sg_player "PlayerData"))

(fn `Save Game `
  (params (Health :type "Float (double-precision)") (Location :type "Vector Structure"))
  (bind _as_bp_sg_player (`self.As BP SG Player`))
  (set `/Game/2DFramework/Blueprints/SaveGame/BP_SG_Player.Health` Health _as_bp_sg_player)
  (set `/Game/2DFramework/Blueprints/SaveGame/BP_SG_Player.Location` Location _as_bp_sg_player)
  (`GameplayStatics.SaveGameToSlot` _as_bp_sg_player "PlayerData"))