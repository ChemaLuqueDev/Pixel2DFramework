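; Enemy attack skills component for the 2D framework, exposing a melee and a ranged attack event.
; Both store the EnemyConfig and line-trace for pawns from the owner along the X component of its forward vector, using the first attack's range plus a width offset.
; On a hit, melee applies that attack's damage to the passed target, while ranged spawns BP_Projectile_Enemy carrying it.
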(event `CS_Melee`
  (params (`Enemy Config` :type "/Game/2DFramework/Data/Structs/Enemy/S_EnemyConfig Structure") (Target :type "Actor Object Reference") (Owner :type "Actor Object Reference") (`Width Trace To Pawn` :type "Float (double-precision)") (`Z-Axis Line Trace To Pawn` :type "Vector Structure"))
  (set `self.Enemy Config` `Enemy Config`)
  (if (`.Hit With Player Pawn?` (`self.Line Trace` Owner `Width Trace To Pawn` `Z-Axis Line Trace To Pawn`))
    (`GameplayStatics.ApplyDamage` Target (`.DamageMount_8_AACA7DEA4D69089337C4FB9B2E41676F` (break `/Game/2DFramework/Data/Structs/Enemy/S_AttackType` (`|GetArrayItem` (`.Attacks_30_B3CA7895462F8F9D918EAD96849BB58B` (break `/Game/2DFramework/Data/Structs/Enemy/S_EnemyConfig` (`self.Enemy Config`)))))))))

(event `CS_AtDistance`
  (params (`Enemy Config` :type "/Game/2DFramework/Data/Structs/Enemy/S_EnemyConfig Structure") (Target :type "Actor Object Reference") (Owner :type "Actor Object Reference") (`Width Trace to Pawn` :type "Float (double-precision)") (`Z-Axis Line Trace to Pawn` :type "Vector Structure") (`Spawn Projectile Location` :type "Vector Structure"))
  (set `self.Enemy Config` `Enemy Config`)
  (if (`.Hit With Player Pawn?` (`self.Line Trace` Owner `Width Trace to Pawn` `Z-Axis Line Trace to Pawn`))
    (`|SpawnActorFromClass` "/Game/2DFramework/Systems/ArtificialIntelligenceSystem/Enemies/BP_Projectile_Enemy.BP_Projectile_Enemy_C" (`KismetMathLibrary.MakeTransform` `Spawn Projectile Location`) "AdjustIfPossibleButAlwaysSpawn" "OverrideRootScale" null 1.0 (`.DamageMount_8_AACA7DEA4D69089337C4FB9B2E41676F` (break `/Game/2DFramework/Data/Structs/Enemy/S_AttackType` (`|GetArrayItem` (`.Attacks_30_B3CA7895462F8F9D918EAD96849BB58B` (break `/Game/2DFramework/Data/Structs/Enemy/S_EnemyConfig` (`self.Enemy Config`)))))) null)))

(fn `Line Trace`
  (params (Target :type "Actor Object Reference") (`Width Trace To Pawn` :type "Float (double-precision)") (`Z-Axis Line Trace To Pawn` :type "Vector Structure"))
  (returns (OutHit :type "HitResult Structure") (`Hit With Player Pawn?` :type Boolean))
  (bind _returnvalue (`Actor.K2_GetActorLocation` Target))
  (bind (_outhit _returnvalue_2) (`KismetSystemLibrary.LineTraceSingleForObjects` :`Start` (+ _returnvalue `Z-Axis Line Trace To Pawn`) :`End` (+ _returnvalue (* (`Actor.GetActorForwardVector` Target) (`KismetMathLibrary.MakeVector` (+ (`.RangeAttack_10_D263A0254BDA8C55E2F3A3A33B2C0B13` (break `/Game/2DFramework/Data/Structs/Enemy/S_AttackType` (`|GetArrayItem` (`.Attacks_30_B3CA7895462F8F9D918EAD96849BB58B` (break `/Game/2DFramework/Data/Structs/Enemy/S_EnemyConfig` (`self.Enemy Config`)))))) `Width Trace To Pawn`))) `Z-Axis Line Trace To Pawn`) :`ObjectTypes` (`|MakeArray` "ObjectTypeQuery3" :!type "EObjectTypeQuery Enum") :`TraceColor` (struct :`R` 1.0 :`G` 0.4534 :`A` 1.0) :`TraceHitColor` (struct :`G` 0.688023 :`B` 1.0 :`A` 1.0))) ; LineTraceForObjects crea una línea que devuelve el primer objeto que encuentre que coincida con uno de los tipos de objetos especificados.
  (return _outhit _returnvalue_2))