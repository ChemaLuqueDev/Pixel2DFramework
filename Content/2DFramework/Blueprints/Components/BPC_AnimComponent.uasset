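; Animation component that picks and plays the flipbook of its owning PaperCharacter in a 2D game.
; Each tick it resolves a state by priority: attack, hurt, dead, falling, then moving or stationary based on X velocity.
; Only when the state changes, it looks up the flipbook and loop setting in FlipbookMap and restarts the sprite's playback.
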(event `self.ReceiveTick`
  (params (DeltaSeconds :type "Float (single-precision)"))
  (`self.Change Animation Status`))

(fn `Change Animation Status`
  (bind (_flipbook _loop_) (break `/Game/2DFramework/Data/Structs/Common/S_AnimConfig` (`BlueprintMapLibrary.Map_Find` (`self.Flipbook Map`) (`self.Status Animation`))))
  (bind _velocity_x (`KismetMathLibrary.BreakVector` (`MovementComponent.Velocity` (`Character.CharacterMovement` (cast `PaperCharacter` (`self.GetOwner`) :!pure true)))))
  (if (`self.Is Attack?`)
    (set `self.New Status Animation` "NewEnumerator3")
    (elif (`self.Is Hurt?`)
      (set `self.New Status Animation` "NewEnumerator7")
      (elif (`self.Is Dead?`)
        (set `self.New Status Animation` "NewEnumerator4")
        (elif (`NavMovementComponent.IsFalling` (`Character.CharacterMovement` (cast `PaperCharacter` (`self.GetOwner`) :!pure true)))
          (set `self.New Status Animation` "NewEnumerator2")
          (elif (!= _velocity_x 0.0)
            (set `self.New Status Animation` "NewEnumerator0")
            (else
              (set `self.New Status Animation` "NewEnumerator5")))))))
  (if (`|EnumInequality` (`self.Status Animation`) (`self.New Status Animation`))
    (set `self.Status Animation` (`self.New Status Animation`))
    (bind _aspaper_character (cast `PaperCharacter` (`self.GetOwner`)))
    (bind _sprite (`PaperCharacter.Sprite` _aspaper_character))
    (`PaperFlipbookComponent.SetFlipbook` _sprite _flipbook)
    (`PaperFlipbookComponent.SetLooping` _sprite _loop_)
    (`PaperFlipbookComponent.PlayFromStart` _sprite)))