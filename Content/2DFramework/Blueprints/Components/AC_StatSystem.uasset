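; Stat component for player and enemies in a 2D game, managing health, mana, armor, experience and levels.
; GetHurt applies armor-scaled damage and can start a looping timer for damage over time, with intervals set by damage type.
; Experience levels up through a data table and updates the HUD.
; Stat changes persist immediately: player stats to the player save, enemy health to a level save map keyed by owner, both restored on BeginPlay.
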(event EventBeginPlay
  (Utilities|FlowControl|Sequence
    (:then_0
      (bind _asbp_gi_main (Utilities|Casting|CastToBP_GI_Main (Game|GetGameInstance)))
      (Variables|🔒SaveGame|Player|SetAs%20BP%20SG%20Player (Variables|/Game/2DFramework/Blueprints/BP_GI_Main.BP_GI_Main_C|GetAs%20BP%20SG%20Player _asbp_gi_main))
      (Variables|🔒SaveGame|Player|SetPlayer%20Slot%20Name (Variables|/Game/2DFramework/Blueprints/BP_GI_Main.BP_GI_Main_C|GetPlayer%20Slot%20Name _asbp_gi_main)))
    (:then_1
      (bind _asbp_gm_2dgame (Utilities|Casting|CastToBP_GM_2DGame (Game|GetGameMode)))
      (Variables|🔒SaveGame|Level|SetAs%20BP%20SG%20Level (Variables|/Game/2DFramework/Blueprints/Core/BP_GM_2DGame.BP_GM_2DGame_C|GetAs%20BP%20SG%20Level _asbp_gm_2dgame))
      (Variables|🔒SaveGame|Level|SetLevel%20Data%20Slot (Variables|/Game/2DFramework/Blueprints/Core/BP_GM_2DGame.BP_GM_2DGame_C|GetLevel%20Data%20Slot _asbp_gm_2dgame)))
    (:then_2
      (InitFunction|InitializeVariables (Variables|💚Health|GetPlayer%20Max%20Health) (Variables|💙Mana|GetMax%20Mana))
      (🔒SaveGame|LoadStats))))

(event Custom|Progressive%20Damage
  (params (Damage :type Float%20%28double-precision%29))
  ;[1 0 0.1422] Progressive Damage
  ; Daño progresivo
  (bind _returnvalue (Utilities|Time|SetTimerbyEvent (delegate Custom|Progressively%20Subtract%20Life) (Variables|⚔Damage|GetTime%20Between%20Progressive%20Damage) true)))

(event Custom|Progressively%20Subtract%20Life
  ;[1 0 0.1422] Progressive Damage
  ; Daño progresivo
  (if (Variables|⚔Damage|GetStill%20Receiving%20Damage?)
    (💚Health|GetHurt true (stale Custom|Progressive%20Damage Damage))
    (else
      (Utilities|Time|ClearandInvalidateTimerbyHandle (stale Custom|Progressive%20Damage _returnvalue)))))

(event Custom|Add%20Health%20|%20Run%20In%20Server
  (params (Still%20Receiving%20Damage? :type Boolean) (Health%20To%20Add :type Float%20%28double-precision%29))
  (CallFunction|AddHealth|RuninClient Still%20Receiving%20Damage? Health%20To%20Add))

(event Custom|Add%20Health%20|%20Run%20In%20Client
  (params (Still%20Receiving%20Damage? :type Boolean) (Health%20To%20Add :type Float%20%28double-precision%29))
  (💚Health|AddHealth Still%20Receiving%20Damage? Health%20To%20Add))

(fn InitializeVariables
  (params (Max%20Health :type Float%20%28double-precision%29) (Max%20Maná :type Float%20%28double-precision%29))
  ;[0.03955 0.6445 0] Health Variables
  ; Variables de Vida
  (Variables|💚Health|SetPlayer%20Max%20Health Max%20Health)
  ;[0 0.4727 1] Maná Variables
  ; Variables de la Maná
  (Variables|💙Mana|SetMax%20Mana Max%20Maná))

(fn SwitchDamage
  (params (Damage%20Type :type Damage%20Type%20Object%20Reference))
  (switch Utilities|FlowControl|Switch|SwitchonE_Damage (.Value (Utilities|Map|Find (Variables|⚔Damage|GetDamage%20Map) (Utilities|GetClass Damage%20Type)))
    (:NewEnumerator0
      (Variables|⚔Damage|SetStill%20Receiving%20Damage? false))
    (:NewEnumerator1
      (Variables|⚔Damage|SetStill%20Receiving%20Damage? true)
      (Variables|⚔Damage|SetTime%20Between%20Progressive%20Damage 5.0))
    (:NewEnumerator2
      (Variables|⚔Damage|SetStill%20Receiving%20Damage? true)
      (Variables|⚔Damage|SetTime%20Between%20Progressive%20Damage 3.0))
    (:NewEnumerator3
      (Variables|⚔Damage|SetStill%20Receiving%20Damage? true)
      (Variables|⚔Damage|SetTime%20Between%20Progressive%20Damage 1.0))))

(fn SetArmor
  (Variables|❤Armor|SetArmor (.Value (Utilities|Map|Find (Variables|❤Armor|GetArmor%20Map) (Variables|❤Armor|GetActual%20Armor%20Equiped)))))

(fn GetNormalizeMana
  (return (/ (Variables|💙Mana|GetMana) (Variables|💙Mana|GetMax%20Mana))))

(fn SubtractMana
  (params (Mana%20To%20Subtract :type Float%20%28double-precision%29))
  (Variables|💙Mana|SetMana (Math|Float|Clamp(Float) (- (Variables|💙Mana|GetMana) Mana%20To%20Subtract) 0.0 (Variables|💙Mana|GetMax%20Mana)))
  (🔒SaveGame|SaveStats)
  (Default|CallOnManaChange self))

(fn AddMana
  (params (Mana%20To%20Add :type Float%20%28double-precision%29))
  (Variables|💙Mana|SetMana (Math|Float|Clamp(Float) (+ (Variables|💙Mana|GetMana) Mana%20To%20Add) 0.0 (Variables|💙Mana|GetMax%20Mana)))
  (🔒SaveGame|SaveStats)
  (Default|CallOnManaChange self))

(fn GetHurt
  (params (Still%20Receiving%20Damage? :type Boolean) (Damage :type Float%20%28double-precision%29))
  (bind _armor_factor (Variables|❤Armor|GetArmor%20Factor))
  (bind _actual_armor_equiped (Variables|❤Armor|GetActual%20Armor%20Equiped))
  (bind _actual_armor_equiped_2 (Variables|❤Armor|GetActual%20Armor%20Equiped))
  (bind _value (Utilities|Map|Find _armor_factor _actual_armor_equiped))
  (bind _returnvalue (== _actual_armor_equiped_2 ""))
  (bind _returnvalue_2 (Math|Conversions|ToFloat(Integer) _value))
  (bind _returnvalue_3 (|(Base_Damage/(1+({9F6129D2-4D70-C762-58C7-3786F682F90A}/(Armor_Factor+0.000100)))) Damage _returnvalue_2))
  (bind _returnvalue_4 (Math|Float|SelectFloat Damage _returnvalue_3 _returnvalue))
  (❤Armor|SetArmor)
  (if (not (Variables|⚔Damage|GetI%20Die?))
    (Variables|⚔Damage|SetStill%20Receiving%20Damage? Still%20Receiving%20Damage?)
    (💚Health|SubtractHealth _returnvalue_4 0.0)
    (if (Variables|⚔Damage|GetStill%20Receiving%20Damage?)
      (CallFunction|ProgressiveDamage _returnvalue_4))))

(fn AddHealth
  (params (Stop%20Progressive%20Damage? :type Boolean) (Health%20To%20Add :type Float%20%28double-precision%29))
  (Variables|⚔Damage|SetStill%20Receiving%20Damage? Stop%20Progressive%20Damage?)
  (Variables|💚Health|SetHealth (Math|Float|Clamp(Float) (+ (Variables|💚Health|GetHealth) Health%20To%20Add) 0.0 (Variables|💚Health|GetPlayer%20Max%20Health)))
  (🔒SaveGame|SaveStats))

(fn SubtractHealth
  (params (Health%20To%20Subtract :type Float%20%28double-precision%29) (Enemy%20Max%20Health :type Float%20%28double-precision%29))
  (Variables|💚Health|SetHealth (Math|Float|Clamp(Float) (- (Variables|💚Health|GetHealth) Health%20To%20Subtract) 0.0 (select (== (Components|GetOwner) (Game|Player|GetPlayerPawn 0)) (Variables|💚Health|GetPlayer%20Max%20Health) Enemy%20Max%20Health)))
  (Default|CallOnHealthChange self)
  (🔒SaveGame|SaveStats)
  (if (<= (Variables|💚Health|GetHealth) 0.0)
    (Default|CallYouHaveDie)
    (Variables|⚔Damage|SetI%20Die? true)))

(fn GetNormalizeHealth
  (return (/ (Variables|💚Health|GetHealth) (Variables|💚Health|GetPlayer%20Max%20Health))))

(fn SaveStats
  (bind _as_bp_sg_player (Variables|🔒SaveGame|Player|GetAs%20BP%20SG%20Player))
  (if (== (Components|GetOwner) (Game|Player|GetPlayerPawn 0))
    (Variables|/Game/2DFramework/Blueprints/SaveGame/BP_SG_Player.BP_SG_Player_C|SetHealth _as_bp_sg_player (Variables|💚Health|GetHealth))
    (Variables|/Game/2DFramework/Blueprints/SaveGame/BP_SG_Player.BP_SG_Player_C|SetExperience _as_bp_sg_player (Variables|💛Experience|GetExperience))
    (Variables|/Game/2DFramework/Blueprints/SaveGame/BP_SG_Player.BP_SG_Player_C|SetLevel _as_bp_sg_player (Variables|💛Experience|GetLevel))
    (Variables|/Game/2DFramework/Blueprints/SaveGame/BP_SG_Player.BP_SG_Player_C|SetMana _as_bp_sg_player (Variables|💙Mana|GetMana))
    (SaveGame|SaveGametoSlot (Variables|🔒SaveGame|Player|GetAs%20BP%20SG%20Player) (Variables|🔒SaveGame|Player|GetPlayer%20Slot%20Name))
    (else
      (Utilities|Map|Add (Variables|/Game/2DFramework/Blueprints/SaveGame/BP_SG_Level.BP_SG_Level_C|GetEnemyHealthMap (Variables|🔒SaveGame|Level|GetAs%20BP%20SG%20Level)) (Utilities|ResolveSoftReference (Components|GetOwner)) (Variables|💚Health|GetHealth))
      (SaveGame|SaveGametoSlot (Variables|🔒SaveGame|Level|GetAs%20BP%20SG%20Level) (Variables|🔒SaveGame|Level|GetLevel%20Data%20Slot)))))

(fn LoadStats
  (bind _returnvalue (Components|GetOwner))
  (bind _as_bp_sg_level (Variables|🔒SaveGame|Level|GetAs%20BP%20SG%20Level))
  (bind _output (Utilities|ResolveSoftReference _returnvalue))
  (bind _enemyhealthmap (Variables|/Game/2DFramework/Blueprints/SaveGame/BP_SG_Level.BP_SG_Level_C|GetEnemyHealthMap _as_bp_sg_level))
  (bind (_value _returnvalue_2) (Utilities|Map|Find _enemyhealthmap _output))
  (if (== (Components|GetOwner) (Game|Player|GetPlayerPawn 0))
    (if (!= (Variables|/Game/2DFramework/Blueprints/SaveGame/BP_SG_Player.BP_SG_Player_C|GetHealth (Variables|🔒SaveGame|Player|GetAs%20BP%20SG%20Player)) 0.0)
      ;[1 1 1] Health
      (Variables|💚Health|SetHealth (Variables|/Game/2DFramework/Blueprints/SaveGame/BP_SG_Player.BP_SG_Player_C|GetHealth (Variables|🔒SaveGame|Player|GetAs%20BP%20SG%20Player)))
      (Default|CallOnHealthChange self)
      ;[1 1 1] Mana
      (Variables|💙Mana|SetMana (Variables|/Game/2DFramework/Blueprints/SaveGame/BP_SG_Player.BP_SG_Player_C|GetMana (Variables|🔒SaveGame|Player|GetAs%20BP%20SG%20Player)))
      (Default|CallOnManaChange self)
      ;[1 1 1] Experience
      (Variables|💛Experience|SetExperience (Variables|/Game/2DFramework/Blueprints/SaveGame/BP_SG_Player.BP_SG_Player_C|GetExperience (Variables|🔒SaveGame|Player|GetAs%20BP%20SG%20Player)))
      (Variables|💛Experience|SetLevel (Variables|/Game/2DFramework/Blueprints/SaveGame/BP_SG_Player.BP_SG_Player_C|GetLevel (Variables|🔒SaveGame|Player|GetAs%20BP%20SG%20Player)))
      (Default|CallOnExperienceChange self)
      ;[1 1 1] Save
      (SaveGame|SaveGametoSlot (Variables|🔒SaveGame|Player|GetAs%20BP%20SG%20Player) (Variables|🔒SaveGame|Player|GetPlayer%20Slot%20Name))
      (bind _asbp_hud_game (Utilities|Casting|CastToBP_HUD_Game (HUD|GetHUD (Game|GetPlayerController 0))))
      (Default|UpdateExpBar (Variables|/Game/2DFramework/Blueprints/Core/BP_HUD_Game.BP_HUD_Game_C|GetWBP%20Game _asbp_hud_game) (Variables|💛Experience|GetExperience) (Variables|💛Experience|GetLevel)))
    (elif _returnvalue_2
      (Variables|💚Health|SetHealth _value)
      (Default|CallOnHealthChange self))))

(fn AddExperience
  (params (Experience :type Float%20%28double-precision%29))
  (Variables|💛Experience|SetExperience (+ (Variables|💛Experience|GetExperience) Experience))
  (bind _returnvalue (Utilities|GetDataTableRow (Variables|💛Experience|GetLevelDataTable) (Utilities|String|StringToName (Utilities|String|ToString(Integer) (Variables|💛Experience|GetLevel))))
    (:then
      (if (>= (Variables|💛Experience|GetExperience) (Utilities|Struct|BreakS_LevelData _returnvalue))
        (Math|Integer|IncrementInt (Variables|💛Experience|GetLevel)
          (:%20%20
            (bind _asbp_hud_game (Utilities|Casting|CastToBP_HUD_Game (HUD|GetHUD (Game|GetPlayerController 0))))
            (Variables|/Game/2DFramework/Blueprints/UI/Player/WBP_Game.WBP_Game_C|SetPlayer%20Level (Variables|/Game/2DFramework/Blueprints/Core/BP_HUD_Game.BP_HUD_Game_C|GetWBP%20Game _asbp_hud_game) (Utilities|Text|ToText(Integer) (Variables|💛Experience|GetLevel)))
            (Default|UpdateExpBar (Variables|/Game/2DFramework/Blueprints/Core/BP_HUD_Game.BP_HUD_Game_C|GetWBP%20Game _asbp_hud_game) (Variables|💛Experience|GetExperience) (Variables|💛Experience|GetLevel))
            (🔒SaveGame|SaveStats)))
        (else
          (bind _asbp_hud_game_2 (Utilities|Casting|CastToBP_HUD_Game (HUD|GetHUD (Game|GetPlayerController 0))))
          (Default|UpdateExpBar (Variables|/Game/2DFramework/Blueprints/Core/BP_HUD_Game.BP_HUD_Game_C|GetWBP%20Game _asbp_hud_game_2) (Variables|💛Experience|GetExperience) (Variables|💛Experience|GetLevel))
          (🔒SaveGame|SaveStats))))))