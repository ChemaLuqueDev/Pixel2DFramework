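; BP_Door is a 2D door in the interaction system that opens and closes through TurnOn and TurnOff events.
; TurnOn shows open left and right sprites on its two Activable components and disables the Box collision so the doorway is passable.
; TurnOff puts the closed-door sprite on Activable1, clears the other sprite and restores query-and-physics collision on the Box.
; Its construction script only runs the parent's.
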(event `/Game/2DFramework/Systems/InteractionSystem/BPI_Activable.Turn Off`
  (`PaperSpriteComponent.SetSprite` (`self.Activable1`) "/Game/2DFramework/Resources/Textures/Interactables/Door/S_ClosedDoor.S_ClosedDoor")
  (`PaperSpriteComponent.SetSprite` (`self.Activable`) null)
  (`PrimitiveComponent.SetCollisionEnabled` (`self.Box`) "QueryAndPhysics"))

(event `/Game/2DFramework/Systems/InteractionSystem/BPI_Activable.Turn On`
  (`PaperSpriteComponent.SetSprite` (`self.Activable1`) "/Game/2DFramework/Resources/Textures/Interactables/Door/S_OpenedDoor_Left.S_OpenedDoor_Left")
  (`PaperSpriteComponent.SetSprite` (`self.Activable`) "/Game/2DFramework/Resources/Textures/Interactables/Door/S_OpenedDoor_Right.S_OpenedDoor_Right")
  (`PrimitiveComponent.SetCollisionEnabled` (`self.Box`) "NoCollision"))

(fn `UserConstructionScript`
  (`parent.UserConstructionScript`))