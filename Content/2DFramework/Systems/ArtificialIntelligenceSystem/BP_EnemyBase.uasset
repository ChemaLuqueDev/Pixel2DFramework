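; Base enemy pawn for the 2D framework, driven by EnemyConfig for patrol, detection, attacks and drops.
; It patrols points until pawn sensing fills a timed detection meter, then uses a cooldown-gated AI move to trigger melee or ranged skills.
; Hits subtract the player's base damage, update UI, knock it back and can set panic mode.
; Death spawns coins and loot, grants experience and destroys the actor.
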(event `self.ReceiveBeginPlay`
  (`|ExecutionSequence`
    (:`then_0`
      (set `self.Enemy Mode` "NewEnumerator0") ; Set patrol mode at game startup
      (set `CharacterMovementComponent.MaxAcceleration` (`.Velocity_21_A6131F8D41DBA0B7063B3E97BC0949F3` (break `/Game/2DFramework/Data/Structs/Enemy/S_EnemyConfig` (`self.Enemy Config`))) (`self.CharacterMovement`))
      ;[0 0.3968 0.8963 0] Create Enemy UI
      (bind _aswbp_enemy_ui (cast `/Game/2DFramework/Blueprints/UI/Enemy/WBP_EnemyUI` (`WidgetComponent.GetWidget` (`self.Widget_EnemyUI`))))
      (bind _output_get (set `self.WBP Enemy HPBar` (`/Game/2DFramework/Blueprints/UI/Enemy/WBP_EnemyUI.WBP_Enemy_HPBar` _aswbp_enemy_ui)))
      (set `/Game/2DFramework/Blueprints/UI/Enemy/WBP_Enemy_HPBar.Enemy Reference` self _output_get)
      (set `self.WBP Enemy Detection` (`/Game/2DFramework/Blueprints/UI/Enemy/WBP_EnemyUI.WBP_EnemyDetection` _aswbp_enemy_ui))
      ;[0.03955 0.6584 0 0] Set Player Damage
      (bind _asbp_ch_pawn_base (cast `/Game/2DFramework/Blueprints/Core/BP_CH_PawnBase` (`GameplayStatics.GetPlayerPawn` 0)))
      (set `self.Player Damage` (`/Game/2DFramework/Blueprints/Core/BP_CH_PawnBase.Player Damage` _asbp_ch_pawn_base)))
    (:`then_1`
      (`self.Init Patrol Mode`))
    (:`then_2`
      (add `/Game/2DFramework/Blueprints/Components/AC_StatSystem.OnHealthChange` (`self.AC_StatSystem`) (`|CreateDelegate` :!event `HealthChange`)))))

(event `self.ReceiveTick`
  (params (DeltaSeconds :type "Float (single-precision)"))
  (`self.Handle Rotation`))

(event `HealthChange`
  (params (`Stat Component` :type "/Game/2DFramework/Blueprints/Components/AC_StatSystem Object Reference"))
  (bind _wbp_enemy_hpbar (`self.WBP Enemy HPBar`)
    (:`then`
      (`/Game/2DFramework/Blueprints/UI/Enemy/WBP_Enemy_HPBar.Update Health Bar` _wbp_enemy_hpbar))
    (:`else`)))

(event `Continue Move To`
  (bind _returnvalue (`GameplayStatics.GetPlayerPawn` 0))
  (bind ((`CooldownAttack_9_2E8449004A5CE771756803BF44EA2943` _cooldownattack) (`RangeAttack_10_D263A0254BDA8C55E2F3A3A33B2C0B13` _rangeattack)) (break `/Game/2DFramework/Data/Structs/Enemy/S_AttackType` (`|GetArrayItem` (`.Attacks_30_B3CA7895462F8F9D918EAD96849BB58B` (break `/Game/2DFramework/Data/Structs/Enemy/S_EnemyConfig` (`self.Enemy Config`))))))
  (`|ExecutionSequence` :!label _label
    (:`then_0`
      (if (`|EnumInequality` (`self.Enemy Mode`) "NewEnumerator2")
        (set `self.Enemy Mode` "NewEnumerator1")
        (set `self.View Pawn?` true)))
    (:`then_1`
      (if (`self.Is Player Detected?`) :!label _label_2
        (`self.Move To`)
        (`KismetSystemLibrary.Delay` _cooldownattack)
        (goto _label_3 :!via `Open`)
        (else
          (set `self.Detection Level` (`.DetectionVelocity_24_2B57E93B474D6355C65826847B5B5F96` (break `/Game/2DFramework/Data/Structs/Enemy/S_EnemyConfig` (`self.Enemy Config`))))
          (`/Game/2DFramework/Blueprints/UI/Enemy/WBP_EnemyDetection.Update Percent Bar` (`self.WBP Enemy Detection`) (/ (`self.Actual Detection Level`) (`self.Detection Level`)) self)
          (if (`self.Distance Player Visible` self)
            (set `self.View Pawn?` true)
            (bind _result (`/Engine/EditorBlueprintResources/StandardMacros.IncrementInt` (`self.Actual Detection Level`))
              (:`  `
                (`KismetSystemLibrary.Delay` 0.2)
                (`self.Set Player Detected` (> _result (`self.Detection Level`)) true)))
            (else
              (set `self.View Pawn?` false)
              (bind _result_2 (`/Engine/EditorBlueprintResources/StandardMacros.DecrementInt` (`self.Actual Detection Level`))
                (:`  `
                  (`KismetSystemLibrary.Delay` 0.2)
                  (`self.Set Player Detected` (< _result_2 1)))))))))
    (:`then_2`
      (if (not (`self.View Pawn?`))
        (`self.Init Patrol Mode`)))))

(event `Move To`
  (bind _returnvalue (`GameplayStatics.GetPlayerPawn` 0))
  (`/Engine/EditorBlueprintResources/StandardMacros.Gate` false :!label _label_3
    (:`Exit`
      (`AITask_MoveTo.AIMoveTo` (`AIBlueprintHelperLibrary.GetAIController` self) (`self.K2_GetActorLocation` _returnvalue) _returnvalue (`.RangeAttack_10_D263A0254BDA8C55E2F3A3A33B2C0B13` (break `/Game/2DFramework/Data/Structs/Enemy/S_AttackType` (`|GetArrayItem` (`.Attacks_30_B3CA7895462F8F9D918EAD96849BB58B` (break `/Game/2DFramework/Data/Structs/Enemy/S_EnemyConfig` (`self.Enemy Config`)))))) "Disable" "Enable" true true false "Enable"
        (:`then`
          (goto _label_3 :!via `Close`))
        (:`OnRequestFailed`
          (set `self.Is Player Detected?` false)
          (`self.Reset Detection`))
        (:`OnMoveFinished`
          (set `self.Stop Move` false)
          (`self.Select Attack`))))))

(event `self.PawnSensing.OnSeePawn`
  (params (Pawn :type "Pawn Object Reference"))
  (if (<= (`KismetMathLibrary.VSize` (- (`self.K2_GetActorLocation` (`GameplayStatics.GetPlayerPawn` 0)) (`self.K2_GetActorLocation`))) (`.DetectionDistance_23_4BBCEAD84915DF03E86F13879812540B` (break `/Game/2DFramework/Data/Structs/Enemy/S_EnemyConfig` (`self.Enemy Config`))))
    (goto _label)
    (else
      (bind _result (`/Engine/EditorBlueprintResources/StandardMacros.DecrementInt` (`self.Actual Detection Level`))
        (:`  `
          (`KismetSystemLibrary.Delay` 0.2)
          (`self.Set Player Detected` (< (`KismetMathLibrary.Clamp` _result 0 (`self.Detection Level`)) 1))
          (set `/Game/2DFramework/Blueprints/Components/BPC_AnimComponent.Is Attack?` false (`self.BPC_AnimComponent`))
          (`self.Continue Move To`))))))

(event `Reset Detection`
  (goto _label_2))

(event `Stop Movement`
  (`MovementComponent.StopMovementImmediately` (`self.CharacterMovement`)))

(event `Handle Rotation`
  (bind _returnvalue_x (`KismetMathLibrary.BreakVector` (`KismetMathLibrary.GetDirectionUnitVector` (`self.K2_GetActorLocation` (`GameplayStatics.GetPlayerCharacter` 0)) (`self.K2_GetActorLocation`))))
  ;[0.4827 0.1124 0.6771 0] Rotate Enemy
  (if (or (`self.View Pawn?`) (`self.Is Hurt?`))
    (if (`self.Is Dead?`)
      _
      (elif (<= _returnvalue_x 0.0)
        (`self.K2_SetActorRotation` (struct))
        (else
          (`self.K2_SetActorRotation` (struct :`Yaw` 180.0)))))))

(event `Spawn Coins`
  ;[1 0.9697 0.2834 0] Spawn Coins
  (for _ (range (+ (`KismetMathLibrary.RandomIntegerInRange` (`self.Minimun Coins`) (`self.Maximum Coins`)) 1))
    (bind _returnvalue (`|SpawnActorFromClass` "/Game/2DFramework/Systems/InventorySystem/Blueprints/BP_Item.BP_Item_C" (`KismetMathLibrary.MakeTransform` (`SceneComponent.K2_GetComponentLocation` (`self.CapsuleComponent`)) (struct) (0.6 0.6 0.6)) "AdjustIfPossibleButAlwaysSpawn" "OverrideRootScale" null false (`KismetArrayLibrary.Array_Random` (`self.Random Items`)) 1 null))
    (`PrimitiveComponent.AddImpulse` (`/Game/2DFramework/Systems/InventorySystem/Blueprints/BP_Item.Box` _returnvalue) (0.0 0.0 50.0) "None" false)))

(event `Death Event`
  ;[0 0 0 0] Death System
  (`self.Spawn Coins`)
  (`self.Death Function`)
  (`/Game/2DFramework/Blueprints/Components/AC_StatSystem.Add Experience` (`/Game/2DFramework/Blueprints/Library/BFL_StatSystem.Find Stat Component` (`GameplayStatics.GetPlayerPawn` 0)) 50.0)
  (`KismetSystemLibrary.Delay` 2.0)
  (`self.K2_DestroyActor`))

(event `self.ReceiveAnyDamage`
  (params (Damage :type "Float (single-precision)") (DamageType :type "DamageType Object Reference") (InstigatedBy :type "Controller Object Reference") (DamageCauser :type "Actor Object Reference"))
  (bind _bpc_animcomponent (`self.BPC_AnimComponent`))
  ;[1 0 0 0.01] Event Any Damage
  (set `self.Damage Received` Damage)
  (set `/Game/2DFramework/Blueprints/Components/BPC_AnimComponent.Is Hurt?` true (`self.BPC_AnimComponent`))
  (set `self.Is Hurt?` true)
  (`self.Handle Rotation`)
  (`/Game/2DFramework/Blueprints/UI/Enemy/WBP_EnemyDetection.Blink Animation` (`self.WBP Enemy Detection`))
  (`self.Create Floating Damage Text`)
  (`AddComponent|NODE_AddNiagaraComponent-0` :`bManualAttachment` true :`RelativeTransform` (`KismetMathLibrary.MakeTransform` (`SceneComponent.K2_GetComponentLocation` (`self.Sprite`)) (struct) (0.6 0.6 0.6)))
  (set `self.Enemy Mode` "NewEnumerator1")
  (if (not (<= (`.MaxHealth_20_07ADF92341A2D1F6AF49639BD158D76A` (break `/Game/2DFramework/Data/Structs/Enemy/S_EnemyConfig` (`self.Enemy Config`))) (`self.Player Damage`)))
    (set `self.Is Hurt?` true))
  (`/Game/2DFramework/Blueprints/Components/AC_StatSystem.Subtract Health` (`self.AC_StatSystem`) (`self.Player Damage`) (`.MaxHealth_20_07ADF92341A2D1F6AF49639BD158D76A` (break `/Game/2DFramework/Data/Structs/Enemy/S_EnemyConfig` (`self.Enemy Config`))))
  (`/Game/2DFramework/Blueprints/UI/Enemy/WBP_Enemy_HPBar.Update Health Bar` (`self.WBP Enemy HPBar`))
  (if (<= (`/Game/2DFramework/Blueprints/Components/AC_StatSystem.Health` (`self.AC_StatSystem`)) 0.0)
    (`self.Death Event`)
    (set `/Game/2DFramework/Blueprints/Components/BPC_AnimComponent.Is Hurt?` false _bpc_animcomponent)
    (set `/Game/2DFramework/Blueprints/Components/BPC_AnimComponent.Is Dead?` true _bpc_animcomponent)
    (else
      (`self.Launch Character`)
      (`KismetSystemLibrary.Delay` 0.8)
      (`MovementComponent.StopMovementImmediately` (`self.CharacterMovement`))
      (set `self.Is Hurt?` false)
      (set `/Game/2DFramework/Blueprints/Components/BPC_AnimComponent.Is Hurt?` false (`self.BPC_AnimComponent`))
      ;[0.7561 0.1107 1] Panic Mode
      (if (<= (`/Game/2DFramework/Blueprints/Components/AC_StatSystem.Health` (`self.AC_StatSystem`)) (/ (`/Game/2DFramework/Blueprints/Components/AC_StatSystem.Player Max Health` (`self.AC_StatSystem`)) 4.0))
        (set `self.Enemy Mode` "NewEnumerator2")))))

(event `Create Floating Damage Text`
  ;[0.7529 0.1912 0.3813 0] Damage Floating Text
  (bind _returnvalue (`|CreateWidget` "/Game/2DFramework/Blueprints/UI/Common/WBP_FloatingText.WBP_FloatingText_C" null (`|FormatText` "-{Damage} HP" (`self.Player Damage`)) (`self.Floating Text Color`)))
  (bind _output_get (set `self.Floating Text` _returnvalue))
  (`UserWidget.AddToViewport` _output_get 0)
  (`UserWidget.SetPositionInViewport` (`self.Floating Text`) (`PlayerController.ProjectWorldLocationToScreen` (`GameplayStatics.GetPlayerController` 0) (`SceneComponent.K2_GetComponentLocation` (`self.Floating Text Position`)) false) true))

(event `Select Attack`
  (if (or (not (`self.Is Dead?`)) (not (`NavMovementComponent.IsFalling` (`self.CharacterMovement`))))
    (for _array_element (`.Attacks_30_B3CA7895462F8F9D918EAD96849BB58B` (break `/Game/2DFramework/Data/Structs/Enemy/S_EnemyConfig` (`self.Enemy Config`)))
      (switch `/Game/2DFramework/Data/Enum/Enemy/E_AttackType` (break `/Game/2DFramework/Data/Structs/Enemy/S_AttackType` _array_element)
        (:`NewEnumerator0`
          (set `/Game/2DFramework/Blueprints/Components/BPC_AnimComponent.Is Attack?` true (`self.BPC_AnimComponent`))
          (`/Game/2DFramework/Blueprints/Components/BPC_Skills.CS_Melee` (`self.BPC_Skills`) (`self.Enemy Config`) (`GameplayStatics.GetPlayerPawn` 0) self (`self.Width Trace to Pawn`) (`self.Z-Axis Line Trace to Pawn`))
          (set `self.Stop Move` true))
        (:`NewEnumerator2`
          (`/Game/2DFramework/Blueprints/Components/BPC_Skills.CS_AtDistance` (`self.BPC_Skills`) (`self.Enemy Config`) (`GameplayStatics.GetPlayerPawn` 0) self (`self.Width Trace to Pawn`) (`self.Z-Axis Line Trace to Pawn`) (`SceneComponent.K2_GetComponentLocation` (`self.InitPoint_Proyectil`))))))))

(event `Init Patrol Mode`
  (bind ((`PatrolPoints_31_66AB0DC240F76C12C165B28B615F55A9` _patrolpoints)) (break `/Game/2DFramework/Data/Structs/Enemy/S_EnemyConfig` (`self.Enemy Config`)))
  (bind (_location _timeinpatrolpoint) (break `/Game/2DFramework/Data/Structs/Enemy/S_PatrolPoints` (`|GetArrayItem` _patrolpoints (`self.Patrol Point ID`))))
  (if (not (`self.View Pawn?`))
    (`|AIMoveTo` self _location null
      (:`OnSuccess`
        (bind _result (`/Engine/EditorBlueprintResources/StandardMacros.IncrementInt` (`self.Patrol Point ID`))
          (:`  `
            (if (== (`KismetArrayLibrary.Array_Length` _patrolpoints) _result)
              (set `self.Patrol Point ID` 0)
              (else
                (`KismetSystemLibrary.Delay` _timeinpatrolpoint)
                (`self.Init Patrol Mode`))))))
      (:`OnFail`
        (`KismetSystemLibrary.Delay` _timeinpatrolpoint)
        (`self.Init Patrol Mode`)))))

(fn `Death Function`
  (set `self.Is Dead?` true)
  (`PrimitiveComponent.SetCollisionProfileName` (`self.CapsuleComponent`) "NoCollision" true)
  (`/Engine/EditorBlueprintResources/StandardMacros.DoOnce` false
    (:`Completed`
      (`AddComponent|NODE_AddNiagaraComponent-2` :`bManualAttachment` true :`RelativeTransform` (`KismetMathLibrary.MakeTransform` (`SceneComponent.K2_GetComponentLocation` (`self.Sprite`)) (struct) (0.6 0.6 0.6)))
      (`MovementComponent.StopMovementImmediately` (`self.CharacterMovement`))
      (`self.DropItems`))))

(fn `Distance Player Visible`
  (params (Enemy :type "/Game/2DFramework/Systems/ArtificialIntelligenceSystem/BP_EnemyBase Object Reference"))
  (returns (`Player Is Visible?` :type Boolean))
  (return (<= (`KismetMathLibrary.VSize` (- (`self.K2_GetActorLocation` (`GameplayStatics.GetPlayerPawn` 0)) (`self.K2_GetActorLocation` Enemy))) (`.DetectionDistance_23_4BBCEAD84915DF03E86F13879812540B` (break `/Game/2DFramework/Data/Structs/Enemy/S_EnemyConfig` (`/Game/2DFramework/Systems/ArtificialIntelligenceSystem/BP_EnemyBase.Enemy Config` Enemy))))))

(fn `DropItems`
  (for _array_element (`.RewardDrop_34_5C895DE141F05C0386BAAA82554EEE34` (break `/Game/2DFramework/Data/Structs/Enemy/S_EnemyConfig` (`self.Enemy Config`)))
    (bind (_item _mindrop _maxdrop) (break `/Game/2DFramework/Data/Structs/Enemy/S_ItemDrops` _array_element))
    (`|GetDataTableRow` "/Game/2DFramework/Systems/InventorySystem/Data/DT_ItemData.DT_ItemData" _item
      (:`then`
        (bind _returnvalue (`KismetMathLibrary.RandomIntegerInRange` _mindrop _maxdrop))
        (for _ (range (+ _returnvalue 1))
          (`|SpawnActorFromClass` "/Game/2DFramework/Systems/InventorySystem/Blueprints/BP_Item.BP_Item_C" (`KismetMathLibrary.MakeTransform` (+ (`SceneComponent.K2_GetComponentLocation` (`self.DropItemLocation`)) (0.0 0.0 25.0))) "AlwaysSpawn" "OverrideRootScale" null false _item _returnvalue null))))))

(fn `HealingEffect`
  (`AddComponent|NODE_AddNiagaraComponent-3` :`bManualAttachment` true :`RelativeTransform` (`KismetMathLibrary.MakeTransform` (`SceneComponent.K2_GetComponentLocation` (`self.Sprite`)) (struct) (0.6 0.6 0.6))))

(fn `Launch Character`
  (bind _returnvalue_x (`KismetMathLibrary.BreakVector` (`KismetMathLibrary.GetDirectionUnitVector` (`self.K2_GetActorLocation` (`GameplayStatics.GetPlayerPawn` 0)) (`self.K2_GetActorLocation`))))
  (`self.LaunchCharacter` (`KismetMathLibrary.MakeVector` (* (select `bool` (< _returnvalue_x 0.0) :`false` -1.0 :`true` 1.0) -500.0))))

(fn `Set Player Detected`
  (params (Condition :type Boolean) (`Is Player Detected?` :type Boolean))
  (if Condition
    (set `self.Is Player Detected?` `Is Player Detected?`)
    (else
      (`self.Reset Detection`)
      (if (not (`self.Is Player Detected?`))
        (`/Engine/EditorBlueprintResources/StandardMacros.DoOnce` false
          (:`Completed`
            (`self.Stop Movement`)))))))

(fn `UserConstructionScript`)