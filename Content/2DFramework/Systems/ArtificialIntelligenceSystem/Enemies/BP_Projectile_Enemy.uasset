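; Enemy projectile that homes in on the player like a guided missile and damages pawns it hits.
; On BeginPlay a timeline moves the Sphere by interpolating from the actor's location toward player pawn 0, fed by the timeline's DeltaTime output.
; Overlapping a BP_CH_PawnBase calls GetHurt on its ACHPSystem, sets the mushroom projectile flipbook and destroys the actor after a short delay.
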(event `self.Sphere.OnComponentBeginOverlap`
  (params (OverlappedComponent :type "PrimitiveComponent Object Reference") (OtherActor :type "Actor Object Reference") (OtherComp :type "PrimitiveComponent Object Reference") (OtherBodyIndex :type Integer) (bFromSweep :type Boolean) (SweepResult :type "HitResult Structure (by ref)"))
  (bind _asbp_ch_pawn_base (cast `/Game/2DFramework/Blueprints/Core/BP_CH_PawnBase` OtherActor))
  (`/Game/2DFramework/Blueprints/Components/AC_StatSystem.Get Hurt` (`/Game/2DFramework/Blueprints/Core/BP_CH_PawnBase.AC_HPSystem` _asbp_ch_pawn_base) false (`self.Damage Amount`))
  (`PaperFlipbookComponent.SetFlipbook` (`self.PaperFlipbook`) "/Game/2DFramework/Resources/Sprites/Enemies/Mushroom/Projectile/FB_Mushroom_Projectile.FB_Mushroom_Projectile")
  (`KismetSystemLibrary.Delay` 0.5)
  (`self.K2_DestroyActor`))

(event `self.ReceiveBeginPlay`
  (bind _sphere (`self.Sphere`))
  (bind (_direction _delta_time) (`Timeline|Timeline_0` :!via `PlayFromStart`)
    (:`Update`
      (`/Engine/EditorBlueprintResources/StandardMacros.IsValid` _sphere
        (:`Is Valid`
          (bind _returnvalue_location (`KismetMathLibrary.BreakTransform` (`KismetMathLibrary.TInterpTo` (`KismetMathLibrary.MakeTransform` (`self.K2_GetActorLocation`)) (`KismetMathLibrary.MakeTransform` (`self.K2_GetActorLocation` (`GameplayStatics.GetPlayerPawn` 0))) _delta_time 1.0)))
          (`SceneComponent.K2_SetWorldLocation` _sphere _returnvalue_location false false))))))

(fn `UserConstructionScript`
  (`parent.UserConstructionScript`))