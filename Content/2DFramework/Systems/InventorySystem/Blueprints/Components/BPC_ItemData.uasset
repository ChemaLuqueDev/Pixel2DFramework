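; BPC_ItemData is an actor component that makes its owner a pickup item for the 2D framework's inventory system.
; On BeginPlay it turns on replication for the owning actor.
; Interactwith passes the item's data table row name and quantity to the player character's inventory component, destroying the owner only if the add succeeds.
; LookAt returns an empty string.
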(event `self.ReceiveBeginPlay`
  (`Actor.SetReplicates` (`self.GetOwner`) true))

(event `/Game/2DFramework/Systems/InventorySystem/Interfaces/BPI_InventoryInteract.InteractWith`
  (params (`Player Character` :type "/Game/2DFramework/Blueprints/Core/BP_CH_PawnBase Object Reference"))
  (bind _bpc_inventorystm (`/Game/2DFramework/Blueprints/Core/BP_CH_PawnBase.BPC_InventorySTM` `Player Character`))
  (bind (_itemid_datatable _itemid_rowname) (break `DataTableRowHandle` (`self.ItemID`)))
  ;[0 0 0 0] Interact
  (`/Engine/EditorBlueprintResources/StandardMacros.IsValid` _bpc_inventorystm
    (:`Is Valid`
      (bind _success (`/Game/2DFramework/Systems/InventorySystem/Blueprints/Components/BPC_InventorySTM.Add To Inventory` _bpc_inventorystm _itemid_rowname (`self.Quantity`)))
      (if _success
        (`Actor.K2_DestroyActor` (`self.GetOwner`))))))

(fn `LookAt`
  (returns (Message :type Text))
  (return ""))