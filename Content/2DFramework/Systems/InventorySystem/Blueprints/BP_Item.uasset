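; BP_Item is a world item for the 2D framework's inventory, showing a "Pick Up" prompt through LookAt.
; The construction script uses ItemName to pull its sprite from DT_ItemData and fills the item data component with row handle and quantity.
; Special items replay a vertical Timeline motion on a looping timer.
; After a short load-order delay, BeginPlay records class and transform in the level SaveGame and saves it; Destroyed records removal without saving.
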(event `Special Item Animation`
  ;[0.4334 1 0.3801] Special Item Animation
  (`KismetSystemLibrary.K2_SetTimerDelegate` (delegate `Anim`) 5.0 true))

(event `Anim`
  (bind (_returnvalue_x _returnvalue_y) (`KismetMathLibrary.BreakVector` (`self.K2_GetActorLocation`)))
  (bind (_returnvalue_x_2 _returnvalue_y_2 _returnvalue_z) (`KismetMathLibrary.BreakVector` (`SceneComponent.K2_GetComponentLocation` (`self.DefaultSceneRoot`))))
  ;[0.4334 1 0.3801] Special Item Animation
  (bind (_direction _z_axis) (`Timeline|Movement` :!via `PlayFromStart`)
    (:`Update`
      (`self.K2_SetActorLocation` (`KismetMathLibrary.MakeVector` _returnvalue_x _returnvalue_y (+ _returnvalue_z _z_axis)) true))))

(event `self.ReceiveBeginPlay`
  (`KismetSystemLibrary.Delay` 0.2) ; The delay is necessary so that the SG Level Data is loaded first, \notherwise it will give error, since it will try to get it when it is not \nyet created.
  (if (`self.Special Item?`)
    (`self.Special Item Animation`)
    (`self.Anim`))
  (bind _asbp_gm_2dgame (cast `/Game/2DFramework/Blueprints/Core/BP_GM_2DGame` (`GameplayStatics.GetGameMode`)))
  (bind _as_bp_sg_level (`/Game/2DFramework/Blueprints/Core/BP_GM_2DGame.As BP SG Level` _asbp_gm_2dgame))
  (`BlueprintMapLibrary.Map_Add` (`/Game/2DFramework/Blueprints/SaveGame/BP_SG_Level.ActorsAdded` _as_bp_sg_level) (`|ConvertAsset` (`GameplayStatics.GetObjectClass` self)) (`self.GetTransform`))
  (`GameplayStatics.SaveGameToSlot` _as_bp_sg_level (`/Game/2DFramework/Blueprints/Core/BP_GM_2DGame.Level Data Slot` _asbp_gm_2dgame)))

(event `self.ReceiveDestroyed`
  ;[0 0 0 0] On Destroy Item
  (bind _asbp_gm_2dgame (cast `/Game/2DFramework/Blueprints/Core/BP_GM_2DGame` (`GameplayStatics.GetGameMode`)))
  (`KismetArrayLibrary.Array_AddUnique` (`/Game/2DFramework/Blueprints/SaveGame/BP_SG_Level.ActorsRemoved` (`/Game/2DFramework/Blueprints/Core/BP_GM_2DGame.As BP SG Level` _asbp_gm_2dgame)) (`|ConvertAsset` self)))

(fn `LookAt`
  (returns (Message :type Text))
  (bind (_itemid_datatable _itemid_rowname) (break `DataTableRowHandle` (`/Game/2DFramework/Systems/InventorySystem/Blueprints/Components/BPC_ItemData.ItemID` (`self.BPC_ItemData`))))
  (bind _returnvalue (`|GetDataTableRow` _itemid_datatable _itemid_rowname)
    (:`then`
      (return (`|FormatText` "Pick Up {item}" (`.Name_3_6C53946244414507F6CC6A88B2CD4871` (break `/Game/2DFramework/Systems/InventorySystem/Data/S_ItemStruct` _returnvalue)))))))

(fn `UserConstructionScript`
  (bind _bpc_itemdata (`self.BPC_ItemData`))
  (bind _returnvalue (`|GetDataTableRow` "/Game/2DFramework/Systems/InventorySystem/Data/DT_ItemData.DT_ItemData" (`self.Item Name`))
    (:`then`
      (`PaperSpriteComponent.SetSprite` (`self.PaperSprite`) (`.ItemSprite_25_056DC490431FB5FD44D64BAD88775E98` (break `/Game/2DFramework/Systems/InventorySystem/Data/S_ItemStruct` _returnvalue)))
      (set `/Game/2DFramework/Systems/InventorySystem/Blueprints/Components/BPC_ItemData.ItemID` (make `DataTableRowHandle` "/Game/2DFramework/Systems/InventorySystem/Data/DT_ItemData.DT_ItemData" (`self.Item Name`)) _bpc_itemdata)
      (set `/Game/2DFramework/Systems/InventorySystem/Blueprints/Components/BPC_ItemData.Quantity` (`self.Item Quantity`) _bpc_itemdata))))