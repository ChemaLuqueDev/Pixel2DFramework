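; BP_InteractableChest is a chest actor in the inventory system that registers itself with the level's save data.
; Shortly after BeginPlay, it adds its class and transform to the game mode's level save object and writes that slot immediately.
; On destruction, it adds itself to the removed-actors list without saving.
; LookAt returns an empty string, and no opening or item logic appears here.
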(event `self.ReceiveBeginPlay`
  (`KismetSystemLibrary.Delay` 0.2)
  (bind _asbp_gm_2dgame (cast `/Game/2DFramework/Blueprints/Core/BP_GM_2DGame` (`GameplayStatics.GetGameMode`)))
  (bind _as_bp_sg_level (`/Game/2DFramework/Blueprints/Core/BP_GM_2DGame.As BP SG Level` _asbp_gm_2dgame))
  (`BlueprintMapLibrary.Map_Add` (`/Game/2DFramework/Blueprints/SaveGame/BP_SG_Level.ActorsAdded` _as_bp_sg_level) (`|ConvertAsset` (`GameplayStatics.GetObjectClass` self)) (`self.GetTransform`))
  (`GameplayStatics.SaveGameToSlot` _as_bp_sg_level (`/Game/2DFramework/Blueprints/Core/BP_GM_2DGame.Level Data Slot` _asbp_gm_2dgame)))

(event `self.ReceiveDestroyed`
  (bind _asbp_gm_2dgame (cast `/Game/2DFramework/Blueprints/Core/BP_GM_2DGame` (`GameplayStatics.GetGameMode`)))
  (`KismetArrayLibrary.Array_AddUnique` (`/Game/2DFramework/Blueprints/SaveGame/BP_SG_Level.ActorsRemoved` (`/Game/2DFramework/Blueprints/Core/BP_GM_2DGame.As BP SG Level` _asbp_gm_2dgame)) (`|ConvertAsset` self)))

(fn `LookAt`
  (returns (Message :type Text))
  (return ""))

(fn `UserConstructionScript`)