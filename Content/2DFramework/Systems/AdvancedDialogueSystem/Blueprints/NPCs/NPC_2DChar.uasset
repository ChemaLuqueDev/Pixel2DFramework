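; NPC_2DChar is an NPC for the 2D framework's dialogue system, with a floating text label set to its character name at construction.
; SetInteractableState shows or hides that label as the interact indicator.
; ConversationClosed restores game-only input and hides the cursor, while OpenStore waits briefly, then enables UI-only input and the cursor without creating any store UI here.
; DoSomething is a stub returning false.
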(event `/Game/2DFramework/Systems/AdvancedDialogueSystem/Blueprints/BPI_Interact.SetInteractableState`
  (params (`CanShowInteract?` :type Boolean))
  (bind _textrender (`self.TextRender`))
  (if `CanShowInteract?`
    (`SceneComponent.SetVisibility` _textrender true false)
    (else
      (`SceneComponent.SetVisibility` _textrender false false))))

(event `/Game/2DFramework/Systems/AdvancedDialogueSystem/Blueprints/BPI_Interact.ConversationClosed`
  (params (`In Mission?` :type Boolean))
  (bind _returnvalue (`GameplayStatics.GetPlayerController` 0))
  (`WidgetBlueprintLibrary.SetInputMode_GameOnly` _returnvalue)
  (set `PlayerController.bShowMouseCursor` false _returnvalue))

(event `/Game/2DFramework/Systems/AdvancedDialogueSystem/Blueprints/BPI_Interact.Open Store`
  (params (`Store Name` :type Name))
  (bind _returnvalue (`GameplayStatics.GetPlayerController` 0))
  (`KismetSystemLibrary.Delay` 0.2)
  (`WidgetBlueprintLibrary.SetInputMode_UIOnlyEx` _returnvalue null)
  (set `PlayerController.bShowMouseCursor` true _returnvalue))

(fn `DoSomething`
  (returns (`Mission Completed?` :type Boolean))
  (return false))

(fn `UserConstructionScript`
  (`TextRenderComponent.K2_SetText` (`self.TextRender`) (`self.CharacterName`)))