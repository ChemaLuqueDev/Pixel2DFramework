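; NPC Blueprint for the Boticary character in the Advanced Dialogue System, offering a conversation and a store.
; Interact stores the instigator and opens a conversation through the ACBoticary component.
; OpenStore calls the parent, creates a W_Store widget for the given store name, then switches the player to UI-only input with a visible mouse cursor.
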(event `/Game/2DFramework/Systems/AdvancedDialogueSystem/Blueprints/BPI_Interact.Interact`
  (params (Instigator :type "Actor Object Reference"))
  (set `self.Interact Instigator` Instigator)
  (`/Game/2DFramework/Systems/AdvancedDialogueSystem/Blueprints/AC_AdvancedDialogueSystem.OpenConversation` (`self.AC_Boticary`) false))

(event `/Game/2DFramework/Systems/AdvancedDialogueSystem/Blueprints/BPI_Interact.Open Store`
  (params (`Store Name` :type Name))
  (bind _returnvalue (`GameplayStatics.GetPlayerController` 0))
  (`parent.Open Store` `Store Name`)
  (bind _returnvalue_2 (`|CreateWidget` "/Game/2DFramework/Systems/Store/W_Store.W_Store_C" null `Store Name`))
  (`UserWidget.AddToViewport` _returnvalue_2 0)
  (`WidgetBlueprintLibrary.SetInputMode_UIOnlyEx` _returnvalue null)
  (set `PlayerController.bShowMouseCursor` true _returnvalue))

(fn `UserConstructionScript`
  (`parent.UserConstructionScript`))