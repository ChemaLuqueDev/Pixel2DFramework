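; Base dialogue component that runs branching conversations through a W_Dialogue widget, with the empty Dialogue function as the script hook.
; Each progression replays Dialogue from the start: AddDialogue returns recorded choices from DialogueProgress or displays an unanswered line.
; Selected options are recorded and trigger a replay; progress can be rewound or cleared.
; Optional audio component plays soft-referenced voice clips, async-loading unloaded ones, and closing notifies the owner.
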(event `self.ReceiveBeginPlay`
  (if (`self.UseAudio?`)
    (bind _returnvalue (`|AddComponentByClass` :`self` (`self.GetOwner`) :`Class` "/Script/Engine.AudioComponent"))
    (set `self.Audio Component` _returnvalue)))

(event `Load Dialogue Audio`
  (params (`Sound Base` :type "SoundBase Soft Object Reference"))
  (bind _object (`|LoadAsset` `Sound Base`)
    (:`then`
      (bind _assound_base (cast `SoundBase` _object))
      (`AudioComponent.SetSound` (`self.Audio Component`) _assound_base)
      (`AudioComponent.Play` (`self.Audio Component`) 0.0))))

(fn `AddDialogue`
  (params (Speaker :type Text) (Dialogue :type Text) (Options :type "Array of Text") (`Dialogue Audio` :type "SoundBase Soft Object Reference") (`Character Image` :type "Texture2D Object Reference"))
  (returns (State :type "/Game/2DFramework/Systems/AdvancedDialogueSystem/Data/E_DialogueState Enum") (OptionIndex :type Integer))
  (bind (_value _returnvalue) (`BlueprintMapLibrary.Map_Find` (`self.DialogueProgress`) (`self.DialogueIndex`)))
  (`/Engine/EditorBlueprintResources/StandardMacros.IncrementInt` (`self.DialogueIndex`)
    (:`  `
      (if _returnvalue
        (return "NewEnumerator0" _value)
        (else
          (`/Game/2DFramework/Systems/AdvancedDialogueSystem/Blueprints/UI/W_Dialogue.Update Dialogue Text` (`self.DialogueWidget`) (`self.DialogueIndex`) (`local.Speaker`) (`local.Dialogue`) (`local.Options`) (`local.Character Image`))
          (`self.Play Dialogue Audio` (`local.Dialogue Audio`))
          (return "NewEnumerator1" 0))))))

(fn `ClearDialogueProgress`
  (`BlueprintMapLibrary.Map_Clear` (`self.DialogueProgress`)))

(fn `CloseConversation`
  (params (`In Mission?` :type Boolean))
  (`Widget.RemoveFromParent` (`self.DialogueWidget`))
  (`AudioComponent.Stop` (`self.Audio Component`))
  (message `/Game/2DFramework/Systems/AdvancedDialogueSystem/Blueprints/BPI_Interact.ConversationClosed` (`self.GetOwner`) `In Mission?`))

(fn `Dialogue`
  (params (`In Mission?` :type Boolean)))

(fn `OpenConversation`
  (params (`In Mission?` :type Boolean))
  (bind _returnvalue (`|CreateWidget` "/Game/2DFramework/Systems/AdvancedDialogueSystem/Blueprints/UI/W_Dialogue.W_Dialogue_C" null self))
  (bind _output_get (set `self.DialogueWidget` _returnvalue))
  (`UserWidget.AddToViewport` _output_get 0)
  (`self.ProgressDialogue` `In Mission?`))

(fn `Play Dialogue Audio`
  (params (`Dialogue Audio` :type "SoundBase Soft Object Reference"))
  (bind _output (`|ConvertAsset` (`local.Dialogue Audio`)))
  (if (`KismetSystemLibrary.IsValidSoftObjectReference` `Dialogue Audio`)
    (`/Engine/EditorBlueprintResources/StandardMacros.IsValid` _output
      (:`Is Valid`
        (`AudioComponent.SetSound` (`self.Audio Component`) _output)
        (`AudioComponent.Play` (`self.Audio Component`) 0.0))
      (:`Is Not Valid`
        (`self.Load Dialogue Audio` `Dialogue Audio`)))))

(fn `ProgressDialogue`
  (params (`In Mission?` :type Boolean))
  (set `self.DialogueIndex` -1)
  (`self.Dialogue` `In Mission?`))

(fn `RemoveDialogueProgress`
  (params (ProgressStep :type Integer))
  (for _index (range (+ ProgressStep 1))
    (`BlueprintMapLibrary.Map_Remove` (`self.DialogueProgress`) (- (`self.DialogueIndex`) _index))))

(fn `SetDialogueTreeIndex`
  (params (`Dialogue Tree Index` :type Integer))
  (set `self.DialogueTreeIndex` `Dialogue Tree Index`)
  (`self.ClearDialogueProgress`))

(fn `UpdateSelectedOption`
  (params (`Progress Index` :type "Integer (by ref)") (`Option Index` :type "Integer (by ref)"))
  (`BlueprintMapLibrary.Map_Add` (`self.DialogueProgress`) `Progress Index` `Option Index`)
  (`self.ProgressDialogue` false))