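; Dialogue component for the Boticary NPC, an apothecary who offers medicine for sale.
; It overrides Dialogue, calls the parent, then builds a branching conversation with AddDialogue nodes, switching on option index and changing the portrait to match mood.
; Choosing to open the store sends OpenStoreMessage to the owner; stealing or leaving draws a scared or angry reply.
; Each branch ends by clearing dialogue progress and closing the conversation.
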(fn `Dialogue`
  (params (`In Mission?` :type Boolean))
  (`parent.Dialogue` `In Mission?`)
  (bind (_state _optionindex) (`self.AddDialogue` "Boticary" "I have the latest in medicine" (`|MakeArray` "I want to see it" "I'd better go" :!type "Text") null "/Game/2DFramework/Resources/Textures/UI/Store/NPCs/T_Boticary_Happy.T_Boticary_Happy"))
  (switch `/Game/2DFramework/Systems/AdvancedDialogueSystem/Data/E_DialogueState` _state
    (:`NewEnumerator0`
      (switch `int` _optionindex
        (:`0`
          (bind (_state_2 _optionindex_2) (`self.AddDialogue` "Boticary" "I welcome that, let me show you...." (`|MakeArray` "Open Store" "Attempt to steal" :!type "Text") null "/Game/2DFramework/Resources/Textures/UI/Store/NPCs/T_Boticary_Happy.T_Boticary_Happy"))
          (switch `/Game/2DFramework/Systems/AdvancedDialogueSystem/Data/E_DialogueState` _state_2
            (:`NewEnumerator0`
              (switch `int` _optionindex_2
                (:`0`
                  (message `/Game/2DFramework/Systems/AdvancedDialogueSystem/Blueprints/BPI_Interact.Open Store` (`self.GetOwner`) "Boticary")
                  (`self.ClearDialogueProgress`)
                  (`self.CloseConversation` false))
                (:`1`
                  (bind (_state_3 _optionindex_3) (`self.AddDialogue` "Boticary" "What did you say? I think I should go" (`|MakeArray` "Sorry..." :!type "Text") null "/Game/2DFramework/Resources/Textures/UI/Store/NPCs/T_Boticary_Scary.T_Boticary_Scary"))
                  (switch `/Game/2DFramework/Systems/AdvancedDialogueSystem/Data/E_DialogueState` _state_3
                    (:`NewEnumerator0`
                      (switch `int` _optionindex_3
                        (:`0`
                          (`self.ClearDialogueProgress`)
                          (`self.CloseConversation` false))))))))))
        (:`1`
          (bind (_state_4 _optionindex_4) (`self.AddDialogue` "Boticary" "Don't waste my time" (`|MakeArray` "Sorry..." :!type "Text") null "/Game/2DFramework/Resources/Textures/UI/Store/NPCs/T_Boticary_Angry.T_Boticary_Angry"))
          (switch `/Game/2DFramework/Systems/AdvancedDialogueSystem/Data/E_DialogueState` _state_4
            (:`NewEnumerator0`
              (switch `int` _optionindex_4
                (:`0`
                  (`self.ClearDialogueProgress`)
                  (`self.CloseConversation` false))))))))))