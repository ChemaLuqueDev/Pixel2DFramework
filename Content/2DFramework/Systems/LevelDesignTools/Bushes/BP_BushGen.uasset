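; BP_BushGen is a 2D level design tool that procedurally builds a bush from Paper2D sprites in its Construction Script.
; It adds Density sprite components, each with a random sprite from a list, X/Y offset and uniform scale within configurable ranges.
; Each sprite's color is a random lerp between two tint colors, with the blend range clamped to 0–1.
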(fn `UserConstructionScript`
  (bind (_tintvariation_x _tintvariation_y) (`KismetMathLibrary.BreakVector2D` (`self.TintVariation`)))
  (bind _maxxdesviation (`self.MaxXDesviation`))
  (bind (_scalevariation_x _scalevariation_y) (`KismetMathLibrary.BreakVector2D` (`self.ScaleVariation`)))
  (bind _maxydesviation (`self.MaxYDesviation`))
  (for _ (range 1 (+ (`self.Density`) 1))
    (bind _returnvalue (`AddComponent|NODE_AddPaperSpriteComponent-0` :`RelativeTransform` (`KismetMathLibrary.MakeTransform` (`KismetMathLibrary.MakeVector` (`KismetMathLibrary.RandomFloatInRange` (* _maxxdesviation -1.0) _maxxdesviation) (`KismetMathLibrary.RandomFloatInRange` (* _maxydesviation -1.0) _maxydesviation)) (struct) (* (1.0 1.0 1.0) (`KismetMathLibrary.RandomFloatInRange` _scalevariation_x _scalevariation_y)))))
    (`KismetArrayLibrary.Array_Add` (`self.Sprites`) (`PaperSpriteComponent.GetSprite` _returnvalue))
    (bind _output_get (set `self.SpriteAux` (`KismetArrayLibrary.Array_Random` (`self.Sprite`))))
    (`PaperSpriteComponent.SetSprite` _returnvalue _output_get)
    (`PaperSpriteComponent.SetSpriteColor` _returnvalue (`KismetMathLibrary.LinearColorLerp` (`self.ColorTintMin`) (`self.ColorTintMax`) (`KismetMathLibrary.RandomFloatInRange` (`KismetMathLibrary.FClamp` _tintvariation_x) (`KismetMathLibrary.FClamp` _tintvariation_y))))))