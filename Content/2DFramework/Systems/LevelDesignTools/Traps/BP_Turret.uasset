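; BP_Turret is a 2D level trap that deploys when a BP_CH_PawnBase enters its box and retracts when it leaves, using one-shot flipbooks.
; While deployed, a looping timer spawns a BP_Projectile facing the side set by TrueLeft.
; A timeline turns the newest projectile into a guided missile, repositioning it each update between the muzzle and player 0's current location through TInterpTo.
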(event `self.Box.OnComponentEndOverlap`
  (params (OverlappedComponent :type "PrimitiveComponent Object Reference") (OtherActor :type "Actor Object Reference") (OtherComp :type "PrimitiveComponent Object Reference") (OtherBodyIndex :type Integer))
  (cast `/Game/2DFramework/Blueprints/Core/BP_CH_PawnBase` OtherActor)
  (`|ExecutionSequence`
    (:`then_0`
      (`self.Set Flipbook` "/Game/2DFramework/Resources/Sprites/Traps/Turret/Deployment/FB_Deployment_Turret_Reverse.FB_Deployment_Turret_Reverse"))
    (:`then_1`
      (`KismetSystemLibrary.K2_ClearAndInvalidateTimerHandle` (stale `self.Box.OnComponentBeginOverlap` _returnvalue)))))

(event `self.Box.OnComponentBeginOverlap`
  (params (OverlappedComponent :type "PrimitiveComponent Object Reference") (OtherActor :type "Actor Object Reference") (OtherComp :type "PrimitiveComponent Object Reference") (OtherBodyIndex :type Integer) (bFromSweep :type Boolean) (SweepResult :type "HitResult Structure (by ref)"))
  (cast `/Game/2DFramework/Blueprints/Core/BP_CH_PawnBase` OtherActor)
  (`|ExecutionSequence`
    (:`then_0`
      (`self.Set Flipbook` "/Game/2DFramework/Resources/Sprites/Traps/Turret/Deployment/FB_Deployment_Turret.FB_Deployment_Turret"))
    (:`then_1`
      (bind _returnvalue (`KismetSystemLibrary.K2_SetTimerDelegate` (delegate `Spawn Fire Arrow`) 1.0 true)))))

(event `Spawn Fire Arrow`
  (bind _returnvalue (`SceneComponent.K2_GetComponentLocation` (`self.Spawn Projectile`)))
  (bind _returnvalue_2 (select `bool` (`self.True == Left`) :`false` (struct :`Yaw` 180.0) :!type "Rotator Structure"))
  (bind _returnvalue_3 (`|SpawnActorFromClass` "/Game/2DFramework/Systems/LevelDesignTools/Traps/BP_Projectile.BP_Projectile_C" (`KismetMathLibrary.MakeTransform` _returnvalue (select `bool` (`self.True == Left`) :`false` (struct :`Yaw` 180.0) :!type "Rotator Structure")) "AdjustIfPossibleButAlwaysSpawn" "OverrideRootScale" null (select `bool` (`self.True == Left`) :`false` -1.0 :`true` 1.0 :!type "Float (single-precision)") 5.0 null))
  (bind (_direction _delta_time) (`Timeline|Timeline_0` :!via `PlayFromStart`)
    (:`Update`
      (`/Engine/EditorBlueprintResources/StandardMacros.IsValid` _returnvalue_3
        (:`Is Valid`
          (bind _returnvalue_location (`KismetMathLibrary.BreakTransform` (`KismetMathLibrary.TInterpTo` (`KismetMathLibrary.MakeTransform` _returnvalue _returnvalue_2) (`KismetMathLibrary.MakeTransform` (`self.K2_GetActorLocation` (`GameplayStatics.GetPlayerPawn` 0)) _returnvalue_2) _delta_time 1.0)))
          (`self.K2_SetActorLocation` _returnvalue_3 _returnvalue_location false false))))))

(fn `Set Flipbook`
  (params (NewFlipbook :type "PaperFlipbook Object Reference"))
  (bind _turret (`self.Turret`))
  (`PaperFlipbookComponent.SetFlipbook` _turret NewFlipbook)
  (`PaperFlipbookComponent.PlayFromStart` _turret)
  (`PaperFlipbookComponent.SetLooping` _turret false))

(fn `UserConstructionScript`)