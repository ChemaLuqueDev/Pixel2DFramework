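; Base one-way platform actor for a 2D game, letting pawns pass up through it and drop back down.
; A BP_CH_PawnBase overlapping the bottom trigger disables collision on the box and sprite; overlapping the top trigger restores query and physics collision.
; Pressing S, bound as a raw key event in the platform itself, also disables that collision.
; Collision toggles on the whole platform, so it affects everything touching it.
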(event `self.BottomCollision.OnComponentBeginOverlap`
  (params (OverlappedComponent :type "PrimitiveComponent Object Reference") (OtherActor :type "Actor Object Reference") (OtherComp :type "PrimitiveComponent Object Reference") (OtherBodyIndex :type Integer) (bFromSweep :type Boolean) (SweepResult :type "HitResult Structure (by ref)"))
  (cast `/Game/2DFramework/Blueprints/Core/BP_CH_PawnBase` OtherActor)
  (`PrimitiveComponent.SetCollisionEnabled` (`self.Box`) "NoCollision")
  (`PrimitiveComponent.SetCollisionEnabled` (`self.PaperSprite`) "NoCollision"))

(event `Key|S`
  (params (Key :type "Key Structure"))
  (:`Pressed`
    (`PrimitiveComponent.SetCollisionEnabled` (`self.Box`) "NoCollision")
    (`PrimitiveComponent.SetCollisionEnabled` (`self.PaperSprite`) "NoCollision")))

(event `self.TopCollision.OnComponentBeginOverlap`
  (params (OverlappedComponent :type "PrimitiveComponent Object Reference") (OtherActor :type "Actor Object Reference") (OtherComp :type "PrimitiveComponent Object Reference") (OtherBodyIndex :type Integer) (bFromSweep :type Boolean) (SweepResult :type "HitResult Structure (by ref)"))
  (cast `/Game/2DFramework/Blueprints/Core/BP_CH_PawnBase` OtherActor)
  (`PrimitiveComponent.SetCollisionEnabled` (`self.Box`) "QueryAndPhysics")
  (`PrimitiveComponent.SetCollisionEnabled` (`self.PaperSprite`) "QueryAndPhysics"))

(fn `UserConstructionScript`)