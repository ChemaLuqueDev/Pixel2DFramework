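; Level design tool for 2D terrain that builds a Width by Height grid of Paper2D sprite components in the Construction Script.
; Each cell maps to a corner, edge or center slot, nine-slice style, to look up sprite variants in TileMap.
; An unseeded random roll against the slot's Chance thresholds picks the variant, so tiles can change on reconstruction.
; The Layer setting decides whether the sprites have collision.
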(fn `Get Next Sprite`
  (params (`Width Index` :type Integer) (`Height Index` :type Integer))
  (returns (Sprite :type "PaperSprite Object Reference"))
  (bind _height (`self.Height`))
  (bind _height_index (`local.Height Index`))
  (bind _width_index (`local.Width Index`))
  (bind _width (`self.Width`))
  (bind _returnvalue (== _height_index (- _height 1)))
  (bind _returnvalue_2 (== _width_index (- _width 1)))
  (bind (_chance _sprite) (break `/Game/2DFramework/Data/Structs/Terrain/S_TileVariant` (`BlueprintMapLibrary.Map_Find` (`self.TileMap`) (`KismetMathLibrary.MakeVector2D` (`KismetMathLibrary.Conv_IntToDouble` (`self.NewHeight`)) (`KismetMathLibrary.Conv_IntToDouble` (`self.NewWidth`))))))
  (set `self.NewHeight` (`KismetMathLibrary.Clamp` (select `bool` (or (== _height_index 0) _returnvalue) :`false` 1 :`true` (select `bool` (and _returnvalue (< _height 3)) :`false` _height_index :`true` 2)) 0 2))
  (set `self.NewWidth` (`KismetMathLibrary.Clamp` (select `bool` (or (== _width_index 0) _returnvalue_2) :`false` 1 :`true` (select `bool` (and _returnvalue_2 (< _width 3)) :`false` _width_index :`true` 2)) 0 2))
  (set `self.RandomNumber` (`KismetMathLibrary.RandomFloatInRange` 0.0 100.0))
  (for (_array_element _array_index) _chance
    (if (< (`self.RandomNumber`) _array_element)
      (return (`|GetArrayItem` _sprite _array_index)))))

(fn `UserConstructionScript`
  ;[0.0137 0.7454 0.4179] Width
  (for _index (range (`self.Width`))
    ;[0.0137 0.7454 0.4179] Height
    (for _index_2 (range (`self.Height`))
      ;[0 0.3712 0.8388] Get Sprite & Add Paper Sprite Component
      (bind _returnvalue (`AddComponent|NODE_AddPaperSpriteComponent-0` :`RelativeTransform` (`KismetMathLibrary.MakeTransform` (+ (* _index (`self.GetActorForwardVector`) (`self.Distance`)) (* _index_2 (`self.GetActorUpVector`) (`self.Distance`) -1.0)) (`self.K2_GetActorRotation`) (5.0 5.0 5.0))))
      (`PaperSpriteComponent.SetSprite` _returnvalue (`self.Get Next Sprite` _index _index_2))
      ;[0 0.5156 0.4214] Collision Preset
      (if (`|EnumEquality` (`self.Layer`) "NewEnumerator1")
        (`PrimitiveComponent.SetCollisionEnabled` _returnvalue "QueryAndPhysics")
        (else
          (`PrimitiveComponent.SetCollisionEnabled` _returnvalue "NoCollision"))))))